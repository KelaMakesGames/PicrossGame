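; Placeable sock bed sprite that extends a parent Blueprint's rotation and pickup collision behavior.
; On construction and on Rotate, it mirrors BoxAnchor along X for rotations other than 0 and 2.
; SetCollision turns four boxes' collision off while picked up and on otherwise, with a debug print.
; Unwired pickup and place collision chains remain in the event graph.
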(event `/Game/WortelsGarden/Core/Sprites/BPI_Grid.Rotate`
  (bind _rotation (`self.Rotation`))
  (`parent.Rotate`)
  (`SceneComponent.SetRelativeScale3D` (`self.BoxAnchor`) (`KismetMathLibrary.SelectVector` (1.0 1.0 1.0) (-1.0 1.0 1.0) (or (== _rotation 0) (== _rotation 2)))))

(fn `SetCollision`
  (`parent.SetCollision`)
  (`PrimitiveComponent.SetCollisionEnabled` (`self.Box`) (select `bool` (`self.isPickedUp?`) :`false` "QueryAndPhysics" :`true` "NoCollision" :!type "ECollisionEnabled Enum"))
  (`PrimitiveComponent.SetCollisionEnabled` (`self.Box1`) (select `bool` (`self.isPickedUp?`) :`false` "QueryAndPhysics" :`true` "NoCollision" :!type "ECollisionEnabled Enum"))
  (`PrimitiveComponent.SetCollisionEnabled` (`self.Box2`) (select `bool` (`self.isPickedUp?`) :`false` "QueryAndPhysics" :`true` "NoCollision" :!type "ECollisionEnabled Enum"))
  (`PrimitiveComponent.SetCollisionEnabled` (`self.Box3`) (select `bool` (`self.isPickedUp?`) :`false` "QueryAndPhysics" :`true` "NoCollision" :!type "ECollisionEnabled Enum"))
  (`KismetSystemLibrary.PrintString` "set collision"))

(fn `UserConstructionScript`
  (bind _rotation (`self.Rotation`))
  (`parent.UserConstructionScript`)
  (`SceneComponent.SetRelativeScale3D` (`self.BoxAnchor`) (`KismetMathLibrary.SelectVector` (1.0 1.0 1.0) (-1.0 1.0 1.0) (or (== _rotation 0) (== _rotation 2)))))