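; Placeable sprite Blueprint for the right-hand above-ground border in WortelsGarden, with six box components.
; Its construction script runs the parent's script, then shifts each box in local space by the negated SpriteOffsett.
; The event graph holds only disabled placeholder events, so the Blueprint adds no runtime logic of its own.
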(fn `UserConstructionScript`
  (`parent.UserConstructionScript`)
  (for _array_element (`|MakeArray` (`self.Box`) (`self.Box1`) (`self.Box2`) (`self.Box3`) (`self.Box4`) (`self.Box5`))
    (`SceneComponent.K2_AddLocalOffset` _array_element (* (`self.SpriteOffsett`) (-1.0 -1.0 -1.0)) false false)))