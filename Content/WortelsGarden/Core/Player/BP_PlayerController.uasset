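; Player controller for the garden game, owning the HUD, hotbar selection, input modes, carrot and energy counts, and pause and inventory menus.
; Selecting a slot switches input mode, starting or stopping item placement or digging; harvest and variation customising are empty stubs.
; Looping timers snap the carried actor or dig selector to the mouse on a grid, refreshing only when it or the player moves.
; SetTimePaused freezes NPC movement and plant growth.
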(event Custom|MovePickedUpActor
  (bind _worldlocation (Game|Player|ConvertMouseLocationToWorldSpace))
  (bind _returnvalue (Game|Player|GetPlayerPawn 0))
  (bind _pickedupactor (Variables|Pickup|GetPickedUpActor))
  (bind _mouseoffset (Variables|Pickup|GetMouseOffset))
  (bind _returnvalue_2 (Transformation|GetActorLocation _returnvalue))
  (bind _returnvalue_3 (+ (.x _worldlocation) (.x _mouseoffset)))
  (bind _returnvalue_4 (+ (.y _worldlocation) (.y _mouseoffset)))
  (bind _out (Utilities|RoundtoClosest50 _returnvalue_3))
  (bind _out_2 (Utilities|RoundtoClosest50 _returnvalue_4))
  (bind _returnvalue_5 (Math|Vector2D|MakeVector2D _out _out_2))
  ;[0.01891 0.01891 0.01891] Move Sprite
  (bind _pickedupactor_2 (Variables|Pickup|GetPickedUpActor)
    (:then
      (Transformation|SetActorLocation _pickedupactor_2 (Math|Vector|MakeVector _out _out_2 (.z (Transformation|GetActorLocation _pickedupactor_2))) false false)
      (if (or (Class|KismetMathLibrary|NotEqualExactlyVector2DVector2D _returnvalue_5 (Variables|Pickup|GetPickedUpLocation)) (Utilities|Operators|NotEqual(!=) _returnvalue_2 (Variables|Pickup|GetPlayerLocation) 1.0))
        (Variables|Pickup|SetPickedUpLocation _returnvalue_5)
        (Variables|Pickup|SetPlayerLocation _returnvalue_2)
        (Class|BPIGrid|UpdatePlacability(Message) _pickedupactor)
        (Class|BPIGrid|UpdateGridColor(Message) _pickedupactor)))
    (:else)))

(event Custom|StartDigging
  ;[0.01891 0.01891 0.01891] Digging
  (bind _returnvalue (Actor|GetActorOfClass "/Game/WortelsGarden/Core/Sprites/BP_DigSelector.BP_DigSelector_C"))
  (bind _output_get (Variables|Dig|SetDigSelector _returnvalue))
  (Utilities|IsValid _output_get
    (:Is%20Valid
      (bind _returnvalue_2 (Utilities|Time|SetTimerbyEvent (delegate Custom|MoveDigSelector) 0.1 true))
      (Variables|Dig|SetDigTimer _returnvalue_2))
    (:Is%20Not%20Valid
      (Development|PrintString "PlayerController > StartDigging > No valid Dig Selector"))))

(event Custom|StopDigging
  ;[0.01891 0.01891 0.01891] Digging
  (Utilities|Time|PauseTimerbyHandle (Variables|Dig|GetDigTimer))
  (bind _digselector (Variables|Dig|GetDigSelector)
    (:then
      (Transformation|SetActorLocation _digselector (Variables|/Game/WortelsGarden/Core/Sprites/BP_DigSelector.BP_DigSelector_C|GetDefaultLocation _digselector) false false))
    (:else)))

(event Custom|StopHarvesting)

(event Custom|StartHarvesting)

(event Custom|MoveDigSelector
  (bind _worldlocation (Game|Player|ConvertMouseLocationToWorldSpace))
  (bind _returnvalue (Game|Player|GetPlayerPawn 0))
  (bind _returnvalue_2 (Transformation|GetActorLocation _returnvalue))
  (bind _out (Utilities|RoundtoClosest100 (.y _worldlocation)))
  (bind _out_2 (Utilities|RoundtoClosest100 (.x _worldlocation)))
  (bind _returnvalue_3 (- _out_2 5e+01))
  (bind _returnvalue_4 (Math|Vector2D|MakeVector2D _returnvalue_3 _out))
  ;[0.01891 0.01891 0.01891] Digging
  (bind _digselector (Variables|Dig|GetDigSelector)
    (:then
      (Transformation|SetActorLocation _digselector (Math|Vector|MakeVector _returnvalue_3 _out (.z (Transformation|GetActorLocation _digselector))) false false)
      (if (or (Class|KismetMathLibrary|NotEqualExactlyVector2DVector2D _returnvalue_4 (Variables|Dig|GetDigSelectorLocation)) (Utilities|Operators|NotEqual(!=) _returnvalue_2 (Variables|Pickup|GetPlayerLocation) 1.0))
        (Variables|Dig|SetDigSelectorLocation _returnvalue_4)
        (Variables|Pickup|SetPlayerLocation _returnvalue_2)
        (Default|UpdateSelector (Variables|Dig|GetDigSelector))))
    (:else)))

(event EventToggleFillMode
  ;[0.01891 0.01891 0.01891] Nonogram
  (Variables|Nonogram|SetFill? (not (Variables|Nonogram|GetFill?))))

(event EventSetFillMode
  (params (Fill? :type Boolean))
  ;[0.01891 0.01891 0.01891] Nonogram
  (Variables|Nonogram|SetFill? Fill?))

(event EventSetTimePaused
  (params (isTimePaused? :type Boolean))
  (bind _outactors (Actor|GetAllActorsOfClass "/Game/WortelsGarden/Core/NPCs/BP_NPC.BP_NPC_C"))
  (for _array_element _outactors
    (Pawn|Components|CharacterMovement|SetMovementMode (Variables|/Script/Engine.Character|GetCharacterMovement _array_element) (select isTimePaused? "MOVE_None" "MOVE_NavWalking") 0))
  (bind _outactors_2 (Actor|GetAllActorsOfClass "/Game/WortelsGarden/Core/Sprites/BP_Sprite_LargePlant.BP_Sprite_LargePlant_C"))
  (for _array_element_2 _outactors_2
    (if isTimePaused?
      (Default|PauseGrowth (Variables|/Game/WortelsGarden/Core/Sprites/BP_Sprite_LargePlant.BP_Sprite_LargePlant_C|GetBP_Component_Growth _array_element_2))
      (else
        (Default|ResumeGrowth (Variables|/Game/WortelsGarden/Core/Sprites/BP_Sprite_LargePlant.BP_Sprite_LargePlant_C|GetBP_Component_Growth _array_element_2)))))
  (Variables|Default|SetisTimePaused? isTimePaused?))

(event EventAddCarrots
  (params (AmountToAdd :type Integer))
  ;[0.01891 0.01891 0.01891] Nonogram
  (Variables|Default|SetCarrots (+ AmountToAdd (Variables|Default|GetCarrots))))

(event EventBeginPlay
  ;[0.01891 0.01891 0.01891] BeginPlay
  (bind _returnvalue (UserInterface|CreateWidget "/Game/WortelsGarden/UI/HUD/WBP_HUD.WBP_HUD_C" self))
  (bind _output_get (Variables|Default|SetHUD _returnvalue))
  (UserInterface|Viewport|AddtoViewport _returnvalue 99)
  (CallFunction|SelectInventoryIndex)
  (Variables|Default|SetbEnableMouseOverEvents true)
  (bind _returnvalue_2 (Utilities|Time|SetTimerbyEvent (delegate Custom|MovePickedUpActor) 0.1 true))
  (bind _output_get_2 (Variables|Pickup|SetPickupTimer _returnvalue_2))
  (Variables|Pickup|GetPickedUpActor
    (:then)
    (:else
      (Utilities|Time|PauseTimerbyHandle _output_get_2))))

(event EventRemoveCarrots
  (params (AmountToRemove :type Integer))
  (Variables|Default|SetCarrots (- (Variables|Default|GetCarrots) AmountToRemove)))

(event EventPlace
  (bind _returnvalue (Game|Player|GetPlayerPawn 0))
  (bind _selectedinventoryindex (Variables|Default|GetSelectedInventoryIndex))
  ;[0.01891 0.01891 0.01891] Move Sprite
  (Class|BPIGrid|UpdateGridColor(Message) (Variables|Pickup|GetPickedUpActor))
  (Variables|Pickup|SetPickedUpActor 0)
  (Utilities|Time|PauseTimerbyHandle (Variables|Pickup|GetPickupTimer))
  (if (Utilities|Enum|Equal(Enum) (Variables|Default|GetInputMode) "NewEnumerator3")
    (Class|BPIInventorySystem|RemovefromContainerbyIndex(Message) _returnvalue _selectedinventoryindex 1)
    (CallFunction|UpdateContainer _selectedinventoryindex false)
    (CallFunction|SelectInventoryIndex _selectedinventoryindex)
    (bind _hasitem_ (Class|BPIInventorySystem|GetInventoryItembyIndex(Message) _returnvalue _selectedinventoryindex))
    (if _hasitem_
      (CallFunction|StartPlacingItem)
      (else
        (CallFunction|SwitchInputMode "NewEnumerator0" false)))))

(event EventPickup
  (params (PickedUpActor :type Actor%20Object%20Reference) (MouseOffset :type Vector%202D%20Structure))
  ;[0.01891 0.01891 0.01891] Move Sprite
  (bind _output_get (Variables|Pickup|SetPickedUpActor PickedUpActor))
  (Utilities|Time|UnpauseTimerbyHandle (Variables|Pickup|GetPickupTimer))
  (Class|BPIGrid|UpdateGridColor(Message) _output_get))

(event EventSetGridShownActor
  (params (Actor :type Actor%20Object%20Reference))
  (Variables|Default|SetGridShownActor Actor))

(event EventUpdateContainer
  (params (IndexToUpdate :type Integer) (UpdateAllIndexes? :type Boolean))
  (Default|UpdateSlot (Variables|Default|GetHUD) IndexToUpdate UpdateAllIndexes?))

(event EventUpdateCurrentHUDSlot
  (CallFunction|SelectInventoryIndex (Variables|Default|GetSelectedInventoryIndex)))

(event Input|ActionEvents|InputActionToggleFillMode
  (params (Key :type Key%20Structure :default "None"))
  ;[0.01891 0.01891 0.01891] Nonogram
  (:Released
    (Variables|Nonogram|SetFill? (not (Variables|Nonogram|GetFill?)))))

(event Input|ActionEvents|InputActionOpenInventoryMenu
  (params (Key :type Key%20Structure :default "None"))
  (:Released
    (Utilities|IsValid (stale _returnvalue)
      (:Is%20Valid
        (if (Widget|IsVisible (stale _returnvalue))
          (Default|CloseWidget (stale _returnvalue))
          (else
            (bind _returnvalue (UserInterface|CreateWidget "/Game/WortelsGarden/UI/Inventory/WBP_InventoryMenu.WBP_InventoryMenu_C" self :!label _label))
            (UserInterface|Viewport|AddtoViewport _returnvalue 0)
            (Default|OpenWidget _returnvalue))))
      (:Is%20Not%20Valid
        (goto _label)))))

(event Input|ActionEvents|InputActionPauseGame
  (params (Key :type Key%20Structure :default "None"))
  (:Released
    (bind _returnvalue (UserInterface|CreateWidget "/Game/WortelsGarden/UI/PauseScreen/WBP_PauseScreen.WBP_PauseScreen_C" self))
    (UserInterface|Viewport|AddtoViewport _returnvalue 0)
    (Default|OpenWidget _returnvalue)))

(event Input|KeyboardEvents|DebugKey1
  (params (Key :type Key%20Structure :default "None") (ActionValue :type Input%20Action%20Value%20Structure))
  (:Released
    (bind _isa (Utilities|FlowControl|FlipFlop)
      (:A
        _)
      (:B
        _))
    (Widget|SetVisibility (Variables|Default|GetHUD) (select _isa "Visible" "Hidden"))))

(event Input|KeyboardEvents|DebugKeyRightBracket
  (params (Key :type Key%20Structure :default "None") (ActionValue :type Input%20Action%20Value%20Structure))
  (:Pressed
    (bind _result (Math|Float|IncrementFloat (Variables|Default|GetEnergy))
      (:%20%20
        (Development|PrintString (Utilities|String|ToString(Float) _result))))))

(event Input|KeyboardEvents|DebugKeyLeftBracket
  (params (Key :type Key%20Structure :default "None") (ActionValue :type Input%20Action%20Value%20Structure))
  (:Pressed
    (bind _result (Math|Float|DecrementFloat (Variables|Default|GetEnergy))
      (:%20%20
        (Development|PrintString (Utilities|String|ToString(Float) _result))))))

(event Input|MouseEvents|RightMouseButton
  (params (Key :type Key%20Structure :default "None"))
  ;[0.01891 0.01891 0.01891] Nonogram
  (:Pressed
    (Variables|Nonogram|SetRMB? true))
  (:Released
    (Variables|Nonogram|SetRMB? false)))

(event Input|KeyboardEvents|8
  (params (Key :type Key%20Structure :default "None"))
  ;[0.01891 0.01891 0.01891] Inventory
  (:Released
    (CallFunction|SelectInventoryIndex 7)))

(event Input|KeyboardEvents|9
  (params (Key :type Key%20Structure :default "None"))
  ;[0.01891 0.01891 0.01891] Inventory
  (:Released
    (CallFunction|SelectInventoryIndex 8)))

(event Input|KeyboardEvents|0
  (params (Key :type Key%20Structure :default "None"))
  ;[0.01891 0.01891 0.01891] Inventory
  (:Released
    (CallFunction|SelectInventoryIndex 9)))

(event Input|MouseEvents|LeftMouseButton
  (params (Key :type Key%20Structure :default "None"))
  (:Pressed
    (Variables|Default|SetClickLocation (.WorldLocation (Game|Player|ConvertMouseLocationToWorldSpace)))))

(event Input|KeyboardEvents|1
  (params (Key :type Key%20Structure :default "None"))
  ;[0.01891 0.01891 0.01891] Inventory
  (:Released
    (CallFunction|SelectInventoryIndex)))

(event Input|KeyboardEvents|2
  (params (Key :type Key%20Structure :default "None"))
  ;[0.01891 0.01891 0.01891] Inventory
  (:Released
    (CallFunction|SelectInventoryIndex 1)))

(event Input|KeyboardEvents|3
  (params (Key :type Key%20Structure :default "None"))
  ;[0.01891 0.01891 0.01891] Inventory
  (:Released
    (CallFunction|SelectInventoryIndex 2)))

(event Input|KeyboardEvents|4
  (params (Key :type Key%20Structure :default "None"))
  ;[0.01891 0.01891 0.01891] Inventory
  (:Released
    (CallFunction|SelectInventoryIndex 3)))

(event Input|KeyboardEvents|5
  (params (Key :type Key%20Structure :default "None"))
  ;[0.01891 0.01891 0.01891] Inventory
  (:Released
    (CallFunction|SelectInventoryIndex 4)))

(event Input|KeyboardEvents|6
  (params (Key :type Key%20Structure :default "None"))
  ;[0.01891 0.01891 0.01891] Inventory
  (:Released
    (CallFunction|SelectInventoryIndex 5)))

(event Input|KeyboardEvents|7
  (params (Key :type Key%20Structure :default "None"))
  ;[0.01891 0.01891 0.01891] Inventory
  (:Released
    (CallFunction|SelectInventoryIndex 6)))

(fn ConstructionScript)

(fn SwitchInputMode
  (params (InputMode :type E_InputModes%20Enum :default "NewEnumerator0") (isNewIndex? :type Boolean))
  (if (or (Utilities|Enum|NotEqual(Enum) InputMode (Variables|Default|GetInputMode)) isNewIndex?)
    (switch Utilities|FlowControl|Switch|SwitchonE_InputModes (Variables|Default|GetInputMode)
      (:NewEnumerator0
        _)
      (:NewEnumerator1
        (CallFunction|StopDigging))
      (:NewEnumerator2
        (CallFunction|StopHarvesting))
      (:NewEnumerator3
        (CallFunction|AbortPlacingItem))
      (:NewEnumerator4
        (CallFunction|StopCustomisingVariation)))
    (bind _output_get (Variables|Default|SetInputMode InputMode))
    (Default|SetKeyInputMode (Variables|Default|GetHUD) _output_get)
    (switch Utilities|FlowControl|Switch|SwitchonE_InputModes _output_get
      (:NewEnumerator1
        (CallFunction|StartDigging))
      (:NewEnumerator2
        (CallFunction|StartHarvesting))
      (:NewEnumerator3
        (CallFunction|StartPlacingItem))
      (:NewEnumerator4
        (CallFunction|StartCustomisingVariation)))))

(fn SelectInventoryIndex
  (params (Index :type Integer))
  (bind _output_get (Variables|Default|SetSelectedInventoryIndex Index))
  (bind (_inputmode _isholdingitem_ _holditem) (Default|SelectIndex (Variables|Default|GetHUD) _output_get))
  (Class|BPIPlayerData|SetHoldItem(Message) (Game|Player|GetPlayerPawn 0) _isholdingitem_ _holditem)
  (CallFunction|SwitchInputMode _inputmode true))

(fn StartPlacingItem
  (bind _returnvalue (Game|Player|GetPlayerPawn 0))
  (bind (_hasitem_ _inventoryitem) (Class|BPIInventorySystem|GetInventoryItembyIndex(Message) _returnvalue (Variables|Default|GetSelectedInventoryIndex)))
  (if _hasitem_
    (if (Utilities|IsValidClass (.Class (Utilities|Struct|BreakS_InventoryItem _inventoryitem)))
      (bind _returnvalue_2 (Game|SpawnActorfromClass (.Class (Utilities|Struct|BreakS_InventoryItem _inventoryitem)) (Math|Transform|MakeTransform "0.000000,3500.000000,0.000000" "0, 0, 0" "1.000000,1.000000,1.000000") "Undefined" "MultiplyWithRoot" 0 _returnvalue))
      (Class|BPISpriteActions|SetVariation(Message) _returnvalue_2 (.Variation (Utilities|Struct|BreakS_InventoryItem _inventoryitem)))
      (Class|BPISpriteActions|UpdateMouseOverGrid(Message) _returnvalue_2)
      (CallFunction|Pickup _returnvalue_2)
      (Class|BPISpriteActions|SetIsPickedUp(Message) _returnvalue_2 true)
      (return (Utilities|IsValid _returnvalue_2))
      (else
        (return false)))
    (else
      (return false))))

(fn AbortPlacingItem
  (bind _pickedupactor (Variables|Pickup|GetPickedUpActor)
    (:then
      (if (not (Game|IsActorBeingDestroyed _pickedupactor))
        (Actor|DestroyActor _pickedupactor)))
    (:else)))

(fn StartCustomisingVariation)

(fn StopCustomisingVariation)

(fn GetNonogramMistakes
  (return))

(fn AddActiveWidget
  (params (Widget :type Widget%20Object%20Reference))
  (return false))

(fn AddtoContainer
  (params (Item :type S%20Inventory%20Item%20Structure))
  (return false 0))

(fn AddtoContainerbyIndex
  (params (Item :type S%20Inventory%20Item%20Structure) (Index :type Integer))
  (return false))

(fn FindEmptyIndex
  (return false 0))

(fn FindinContainer
  (params (Name :type Name :default "None") (Variation :type Integer))
  (return false 0))

(fn GetActiveWidgets
  (return 0))

(fn GetActorRotatability
  (return false false))

(fn GetCarrots
  (return (Variables|Default|GetCarrots)))

(fn GetContainer
  (return 0))

(fn GetDigLocation
  (return (Variables|Dig|GetDigSelectorLocation)))

(fn GetEnergy
  (return (Variables|Default|GetEnergy)))

(fn GetFillMode
  (return (Variables|Nonogram|GetFill?)))

(fn GetGridShownActor
  (return (Variables|Default|GetGridShownActor)))

(fn GethasPickedUpActor?
  (return (Utilities|Time|IsTimerActivebyHandle (Variables|Pickup|GetPickupTimer))))

(fn GetHUDWidget
  (return (Variables|Default|GetHUD)))

(fn GetInputMode
  (return (Variables|Default|GetInputMode)))

(fn GetInventory
  (return 0))

(fn GetInventoryItembyIndex
  (params (Index :type Integer))
  (return false ""))

(fn GetIsContainerFull
  (return false))

(fn GetisPickedUp?
  (return false))

(fn GetNonogramDifficultyLevel
  (return (Variables|Nonogram|GetDifficultyLevel)))

(fn GetPickedUpActor
  (bind _pickedupactor (Variables|Pickup|GetPickedUpActor))
  (return _pickedupactor (Utilities|IsValid _pickedupactor)))

(fn GetRMB
  (return (Variables|Nonogram|GetRMB?)))

(fn GetShouldGamePause
  (return false))

(fn GetTimePaused?
  (return (Variables|Default|GetisTimePaused?)))

(fn GetZoomSensitivity
  (return (Variables|Settings|GetZoomSensitivity)))

(fn RemoveActiveWidget
  (params (Widget :type Widget%20Object%20Reference))
  (return false))

(fn RemoveEnergy
  (params (EnergyToRemove :type Float%20%28double-precision%29))
  (bind _output_get (Variables|Default|SetEnergy (Math|Float|Clamp(Float) (- (Variables|Default|GetEnergy) EnergyToRemove) 0.0 1e+01)))
  (if (< _output_get 0.5)
    (bind _asbp_wortel (Utilities|Casting|CastToBP_Wortel (Game|Player|GetPlayerPawn 0)))
    (Rendering|SetVisibility (Variables|/Game/WortelsGarden/Core/Player/BP_Wortel.BP_Wortel_C|GetEmote _asbp_wortel) true false)
    (return _output_get)))

(fn RemovefromContainer
  (params (Name :type Name :default "None") (Variation :type Integer) (Amount :type Integer))
  (return false 0))

(fn RemovefromContainerbyIndex
  (params (Index :type Integer) (Amount :type Integer))
  (return 0))