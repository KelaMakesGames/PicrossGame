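; BP_Wortel is the player character: it handles movement, ortho camera zoom, interaction, held-item display and eating food for energy.
; Overlap spheres notify nearby grid actors and rotate sprites, while interface functions expose the inventory container, dialogue and interactable list.
; An active-widget stack drives focus and game pause.
; Clothing child actors animate from a data table, sharing the body's sort priority, which line traces switch when underground.
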(event `self.ReceiveBeginPlay`
  ;[0.01891 0.01891 0.01891] BeginPlay
  (for _array_element (`PrimitiveComponent.GetOverlappingActors` (`self.GridInteractableSphere`) "/Game/WortelsGarden/Core/Sprites/BP_Sprite.BP_Sprite_C")
    (message `/Game/WortelsGarden/Core/Sprites/BPI_Grid.SetInGridInteractableRange` _array_element true)))

(event `InputAxis|MoveRight`
  (params (AxisValue :type "Float (single-precision)"))
  ;[0.01891 0.01891 0.01891] Input
  (`self.AddMovementInput` (`KismetMathLibrary.MakeVector` AxisValue)))

(event `InputAxis|MoveBack`
  (params (AxisValue :type "Float (single-precision)"))
  ;[0.01891 0.01891 0.01891] Input
  (`self.AddMovementInput` (`KismetMathLibrary.MakeVector` 0.0 AxisValue))
  (`self.CheckUnderground`))

(event `self.GridInteractableSphere.OnComponentBeginOverlap`
  (params (OverlappedComponent :type "PrimitiveComponent Object Reference") (OtherActor :type "Actor Object Reference") (OtherComp :type "PrimitiveComponent Object Reference") (OtherBodyIndex :type Integer) (bFromSweep :type Boolean) (SweepResult :type "HitResult Structure (by ref)"))
  ;[0.01891 0.01891 0.01891] Interactables
  (message `/Game/WortelsGarden/Core/Sprites/BPI_Grid.SetInGridInteractableRange` OtherActor true))

(event `InputAxisKey|MouseWheelAxis`
  (params (AxisValue :type "Float (single-precision)"))
  (bind _camera (`self.Camera`))
  ;[0.01891 0.01891 0.01891] Interactables
  (if (!= AxisValue 0.0)
    (bind _zoomsensitivity (message `/Game/WortelsGarden/Core/Player/BPI_PlayerData.GetZoomSensitivity` (`GameplayStatics.GetPlayerController` 0)))
    (`CameraComponent.SetOrthoWidth` _camera (`KismetMathLibrary.FClamp` (+ (* (* AxisValue 4.0) _zoomsensitivity) (`CameraComponent.OrthoWidth` _camera)) 300.0 2300.0))))

(event `self.GridInteractableSphere.OnComponentEndOverlap`
  (params (OverlappedComponent :type "PrimitiveComponent Object Reference") (OtherActor :type "Actor Object Reference") (OtherComp :type "PrimitiveComponent Object Reference") (OtherBodyIndex :type Integer))
  ;[0.01891 0.01891 0.01891] Interactables
  (message `/Game/WortelsGarden/Core/Sprites/BPI_Grid.SetInGridInteractableRange` OtherActor false))

(event `Key|RightMouseButton`
  (params (Key :type "Key Structure"))
  (bind _returnvalue (`GameplayStatics.GetPlayerController` 0))
  ;[0.01891 0.01891 0.01891] Interactables
  (:`Released`
    (bind _haspickedupactor_ (message `/Game/WortelsGarden/Core/Player/BPI_PlayerData.GethasPickedUpActor?` _returnvalue :!label _label))
    (if (not _haspickedupactor_)
      (bind _gridshownactor (message `/Game/WortelsGarden/Core/Player/BPI_PlayerData.GetGridShownActor` _returnvalue))
      (`/Engine/EditorBlueprintResources/StandardMacros.IsValid` _gridshownactor
        (:`Is Valid`
          (bind (_canrotate_ _canmirror_) (message `/Game/WortelsGarden/Core/Sprites/BPI_Grid.GetActorRotatability` _gridshownactor))
          (if (not (or _canrotate_ _canmirror_))
            (`CameraComponent.SetOrthoWidth` (`self.Camera`) 900.0 :!label _label_2)))
        (:`Is Not Valid`
          (goto _label_2))))))

(event `Key|MiddleMouseButton`
  (params (Key :type "Key Structure"))
  ;[0.01891 0.01891 0.01891] Interactables
  (:`Released`
    (goto _label)))

(event `self.RotateSpriteSphere.OnComponentBeginOverlap`
  (params (OverlappedComponent :type "PrimitiveComponent Object Reference") (OtherActor :type "Actor Object Reference") (OtherComp :type "PrimitiveComponent Object Reference") (OtherBodyIndex :type Integer) (bFromSweep :type Boolean) (SweepResult :type "HitResult Structure (by ref)"))
  ;[0.01891 0.01891 0.01891] Interactables
  (message `/Game/WortelsGarden/Core/Sprites/BPI_SpriteActions.RotateSprite` OtherActor))

(event `/Game/WortelsGarden/Core/Player/BPI_PlayerData.SetHoldItem`
  (params (`isHoldingItem?` :type Boolean) (HoldItem :type "PaperSprite Object Reference"))
  (bind _output_get (set `self.HoldItem` HoldItem))
  (`PaperSpriteComponent.SetSprite` (`self.HoldItemSprite`) _output_get)
  (bind _output_get_2 (set `self.isHoldingItem?` `isHoldingItem?`))
  (`SceneComponent.SetVisibility` (`self.HoldItemSprite`) _output_get_2 false))

(event `InputAction|Interact`
  (params (Key :type "Key Structure"))
  (:`Released`
    (if (not (`self.inDialogue?`))
      (message `/Game/WortelsGarden/Core/Player/BPI_Interact.Interact` (`self.ActiveInteractable`)))))

(event `/Game/WortelsGarden/UI/Dialogue/BPI_Dialogue.StartDialogueWithNPC`
  (params (Dialogue :type "DlgDialogue Object Reference") (NPC :type "Object Object Reference"))
  (bind _returnvalue (`DlgManager.StartDialogue` Dialogue (`|MakeArray` NPC (`GameplayStatics.GetPlayerPawn` 0) :!type "Object Object Reference")))
  (set `self.DialogueContext` _returnvalue))

(event `/Game/WortelsGarden/UI/Dialogue/BPI_Dialogue.SelectDialogueOption`
  (params (OptionIndex :type Integer))
  (bind _dialoguecontext (`self.DialogueContext`))
  (bind _dialoguewidget (`self.DialogueWidget`))
  (`/Engine/EditorBlueprintResources/StandardMacros.IsValid` _dialoguecontext
    (:`Is Valid`
      (if (`DlgContext.IsValidOptionIndex` _dialoguecontext OptionIndex)
        (bind _returnvalue (`DlgContext.ChooseOption` (`self.DialogueContext`) OptionIndex))
        (if _returnvalue
          (message `/Game/WortelsGarden/UI/BPI_WidgetInteract.UpdateWidget` _dialoguewidget)
          (else
            (set `self.DialogueContext` null)
            (set `self.inDialogue?` false)
            (message `/Game/WortelsGarden/UI/BPI_WidgetInteract.CloseWidget` _dialoguewidget)))
        (else
          (`KismetSystemLibrary.PrintString` "SelectDialogueOption > Invalid Index given"))))
    (:`Is Not Valid`
      (`KismetSystemLibrary.PrintString` "SelectDialogueOption > Invalid Dlg Context"))))

(event `/Game/WortelsGarden/UI/Dialogue/BPI_Dialogue.SetDialogueWidget`
  (params (DialogueWidget :type "Widget Object Reference"))
  (set `self.DialogueWidget` DialogueWidget))

(event `/Game/WortelsGarden/UI/Dialogue/BPI_Dialogue.SetInDialogue`
  (params (`inDialogue?` :type Boolean))
  (set `self.inDialogue?` `inDialogue?`))

(event `/Game/WortelsGarden/UI/BPI_WidgetInteract.UpdateActiveWidget`
  (bind _returnvalue (`GameplayStatics.GetPlayerController` 0))
  (bind _activewidgets (`self.ActiveWidgets`))
  (bind _output (`|GetArrayItem` _activewidgets (`KismetArrayLibrary.Array_LastIndex` _activewidgets)))
  (if (> (`KismetArrayLibrary.Array_Length` _activewidgets) 0)
    (message `/Game/WortelsGarden/UI/BPI_WidgetInteract.SetFocusToWidget` _output)
    (`KismetSystemLibrary.PrintString` "setting focus to widget (UNPRVEN)")
    (bind _pausegame_ (message `/Game/WortelsGarden/UI/BPI_WidgetInteract.GetShouldGamePause` _output))
    (`GameplayStatics.SetGamePaused` _pausegame_)
    (else
      (bind _hud (message `/Game/WortelsGarden/UI/BPI_WidgetInteract.GetHUDWidget` _returnvalue))
      (message `/Game/WortelsGarden/UI/BPI_WidgetInteract.SetWidgetVisibility` _hud "HitTestInvisible")
      (message `/Game/WortelsGarden/UI/BPI_WidgetInteract.UpdateWidget` _hud)
      (`WidgetBlueprintLibrary.SetInputMode_GameAndUIEx` _returnvalue null "LockOnCapture" false)
      (`GameplayStatics.SetGamePaused` false))))

(event `self.HoldItemSprite.OnClicked`
  (params (TouchedComponent :type "PrimitiveComponent Object Reference") (ButtonPressed :type "Key Structure"))
  (`KismetSystemLibrary.PrintString` "click hold item")
  (bind _asbp_player_controller (cast `/Game/WortelsGarden/Core/Player/BP_PlayerController` (`GameplayStatics.GetPlayerController` 0)))
  (bind _selectedinventoryindex (`/Game/WortelsGarden/Core/Player/BP_PlayerController.SelectedInventoryIndex` _asbp_player_controller))
  (bind (_hasitem_ _inventoryitem) (`self.GetInventoryItemByIndex` _selectedinventoryindex))
  (switch `/Game/WortelsGarden/Core/InventorySystem/E_ItemType` (`.ItemType_34_68274A06D8418B35158C9989C977542C` (break `/Game/WortelsGarden/Core/InventorySystem/S_InventoryItem` _inventoryitem))
    (:`NewEnumerator2`
      _)
    (:`NewEnumerator4`
      _))
  (`KismetSystemLibrary.PrintString` "EAT")
  (bind _ateitem_ (`self.EatInventoryItem` _selectedinventoryindex))
  (`KismetSystemLibrary.PrintString` (select `bool` _ateitem_ :`false` "NO eat" :`true` "YES eat")))

(fn `AddActiveWidget`
  (params (Widget :type "Widget Object Reference"))
  (returns (`success?` :type Boolean))
  (bind _activewidgets (`self.ActiveWidgets`))
  (bind _returnvalue (`KismetArrayLibrary.Array_AddUnique` _activewidgets Widget))
  (bind _pausegame_ (message `/Game/WortelsGarden/UI/BPI_WidgetInteract.GetShouldGamePause` Widget))
  (`GameplayStatics.SetGamePaused` _pausegame_)
  (return (`KismetArrayLibrary.Array_IsValidIndex` _activewidgets _returnvalue)))

(fn `AddInteractable`
  (params (Actor :type "Actor Object Reference") (`SetActive?` :type Boolean))
  (returns (`success?` :type Boolean))
  (`KismetArrayLibrary.Array_AddUnique` (`self.Interactables`) Actor)
  (if `SetActive?`
    (set `self.ActiveInteractable` Actor))
  (return true))

(fn `AddToContainer`
  (params (Item :type "/Game/WortelsGarden/Core/InventorySystem/S_InventoryItem Structure"))
  (returns (`success?` :type Boolean) (Index :type Integer))
  (bind (_success_ _index) (`/Game/WortelsGarden/Core/InventorySystem/BP_Component_Container.AddToInventory` (`self.BP_Component_Container`) Item))
  (return _success_ _index))

(fn `AddToContainerByIndex`
  (params (Item :type "/Game/WortelsGarden/Core/InventorySystem/S_InventoryItem Structure") (Index :type Integer))
  (returns (`success?` :type Boolean))
  (bind _success_ (`/Game/WortelsGarden/Core/InventorySystem/BP_Component_Container.AddToInventoryByIndex` (`self.BP_Component_Container`) Item Index))
  (return _success_))

(fn `CheckCondition`
  (params (Context :type "DlgContext Object Reference") (ConditionName :type Name))
  (returns (ReturnValue :type Boolean))
  (return false))

(fn `CheckUnderground`
  (locals (NewLocalVar :type "Vector Structure" :default (0.0 0.0 0.0)))
  (bind (_returnvalue_x _returnvalue_y) (`KismetMathLibrary.BreakVector` (`self.K2_GetActorLocation`)))
  (bind _sprite (`self.Sprite`))
  (bind _returnvalue (- _returnvalue_y 70.0))
  (bind _returnvalue_2 (+ _returnvalue_x 25.0))
  (bind _returnvalue_3 (- _returnvalue_x 25.0))
  (if (> _returnvalue_y 600.0)
    (bind (_outhit _returnvalue_4) (`KismetSystemLibrary.LineTraceSingle` :`Start` (`KismetMathLibrary.MakeVector` _returnvalue_3 _returnvalue 100.0) :`End` (`KismetMathLibrary.MakeVector` _returnvalue_3 _returnvalue -100.0) :`TraceChannel` "TraceTypeQuery5" :`DrawDebugType` "ForDuration" :`DrawTime` 0.1)) ; top left of player
    (bind (_outhit_2 _returnvalue_5) (`KismetSystemLibrary.LineTraceSingle` :`Start` (`KismetMathLibrary.MakeVector` _returnvalue_2 _returnvalue 100.0) :`End` (`KismetMathLibrary.MakeVector` _returnvalue_2 _returnvalue -100.0) :`TraceChannel` "TraceTypeQuery5" :`DrawDebugType` "ForDuration" :`DrawTime` 0.1)) ; top right of player
    (bind _returnvalue_6 (`KismetMathLibrary.SelectInt` 10 0 (`KismetMathLibrary.BooleanNAND` _returnvalue_5 _returnvalue_4)))
    (if (!= (`PrimitiveComponent.TranslucencySortPriority` _sprite) _returnvalue_6)
      (`PrimitiveComponent.SetTranslucentSortPriority` _sprite _returnvalue_6)
      (`KismetSystemLibrary.PrintString` (`KismetStringLibrary.Conv_IntToString` _returnvalue_6))
      (for _array_element (`|MakeArray` (`self.Clothing`) (`self.Clothing1`) (`self.Clothing2`))
        (bind _asbp_clothing (cast `/Game/WortelsGarden/Core/Player/BP_Clothing` (`ChildActorComponent.ChildActor` _array_element)))
        (`/Game/WortelsGarden/Core/Player/BP_Clothing.SetSortPriority` _asbp_clothing _returnvalue_6)))))

(fn `EatInventoryItem`
  (params (InventoryIndex :type Integer) (`eatWhenNotHungry?` :type Boolean))
  (returns (`AteItem?` :type Boolean))
  (bind (_hasitem_ _inventoryitem) (`self.GetInventoryItemByIndex` InventoryIndex))
  (bind ((`Name_11_3B3AAA62F34C78C7B0F22EA2965F892E` _name) (`ItemType_34_68274A06D8418B35158C9989C977542C` _itemtype)) (break `/Game/WortelsGarden/Core/InventorySystem/S_InventoryItem` _inventoryitem))
  (if (or (`|EnumEquality` _itemtype "NewEnumerator2") (`|EnumEquality` _itemtype "NewEnumerator4"))
    (bind _asbp_player_controller (cast `/Game/WortelsGarden/Core/Player/BP_PlayerController` (`GameplayStatics.GetPlayerController` 0))
      (:`then`
        (bind _energy (`/Game/WortelsGarden/Core/Player/BP_PlayerController.Energy` _asbp_player_controller))
        (if (or (< _energy 10.0) `eatWhenNotHungry?`)
          (bind _returnvalue (`|GetDataTableRow` "/Game/WortelsGarden/Core/InventorySystem/DT_EdibleItems.DT_EdibleItems" _name)
            (:`then`
              (set `/Game/WortelsGarden/Core/Player/BP_PlayerController.Energy` (+ _energy (`.EnergyEffect_6_0E8FFF75D24396AE621E44802222215B` (break `/Game/WortelsGarden/Core/InventorySystem/S_EdibleItem` _returnvalue))) _asbp_player_controller)
              (`self.RemoveFromContainerByIndex` InventoryIndex 1)
              (return true))
            (:`RowNotFound`
              _))))
      (:`CastFailed`
        _)))
  (return false))

(fn `FindEmptyIndex`
  (returns (`foundIndex?` :type Boolean) (Index :type Integer))
  (bind (_foundindex_ _index) (`/Game/WortelsGarden/Core/InventorySystem/BP_Component_Container.FindEmptyIndex` (`self.BP_Component_Container`)))
  (return _foundindex_ _index))

(fn `FindInContainer`
  (params (Name :type Name) (Variation :type Integer))
  (returns (`isFound?` :type Boolean) (ItemIndex :type Integer))
  (bind (_isfound_ _itemindex) (`/Game/WortelsGarden/Core/InventorySystem/BP_Component_Container.FindInInventory` (`self.BP_Component_Container`) Name Variation))
  (return _isfound_ _itemindex))

(fn `GetActiveWidgets`
  (returns (ActiveWidgets :type "Array of Widget Object Reference"))
  (return (`self.ActiveWidgets`)))

(fn `GetBoolValue`
  (params (ValueName :type Name))
  (returns (ReturnValue :type Boolean))
  (return false))

(fn `GetCarrots`
  (returns (Carrots :type Integer))
  (return 0))

(fn `GetContainer`
  (returns (Container :type "/Game/WortelsGarden/Core/InventorySystem/BP_Component_Container Object Reference"))
  (return (`self.BP_Component_Container`)))

(fn `GetDialogueContext`
  (returns (DialogueContext :type "DlgContext Object Reference"))
  (return (`self.DialogueContext`)))

(fn `GetDialogueWidget`
  (returns (DialogueWidget :type "Widget Object Reference"))
  (return null))

(fn `GetDigLocation`
  (returns (DigLocation :type "Vector2D Structure"))
  (return (0.0 0.0)))

(fn `GetEnergy`
  (returns (Energy :type "Float (double-precision)"))
  (return 0.0))

(fn `GetFillMode`
  (returns (`Fill?` :type Boolean))
  (return false))

(fn `GetFloatValue`
  (params (ValueName :type Name))
  (returns (ReturnValue :type "Float (single-precision)"))
  (return 0.0))

(fn `GetGridShownActor`
  (returns (GridShownActor :type "Actor Object Reference"))
  (return null))

(fn `GethasPickedUpActor?`
  (returns (`hasPickedUpActor?` :type Boolean))
  (return false))

(fn `GetHUDWidget`
  (returns (HUD :type "Widget Object Reference"))
  (return null))

(fn `GetInDialgoue`
  (returns (`inDialogue?` :type Boolean))
  (return (`self.inDialogue?`)))

(fn `GetInputMode`
  (returns (InputMode :type "/Game/WortelsGarden/Core/Player/E_InputModes Enum"))
  (return "NewEnumerator0"))

(fn `GetInteractable`
  (returns (ActiveInteractable :type "Actor Object Reference") (Interactables :type "Array of Actor Object Reference"))
  (return (`self.ActiveInteractable`) (`self.Interactables`)))

(fn `GetIntValue`
  (params (ValueName :type Name))
  (returns (ReturnValue :type Integer))
  (return 0))

(fn `GetInventory`
  (returns (Inventory :type "Array of /Game/WortelsGarden/Core/InventorySystem/S_InventoryItem Structure"))
  (return (`/Game/WortelsGarden/Core/InventorySystem/BP_Component_Container.Inventory` (`self.BP_Component_Container`))))

(fn `GetInventoryItemByIndex`
  (params (Index :type Integer))
  (returns (`hasItem?` :type Boolean) (InventoryItem :type "/Game/WortelsGarden/Core/InventorySystem/S_InventoryItem Structure"))
  (bind _inventory (`/Game/WortelsGarden/Core/InventorySystem/BP_Component_Container.Inventory` (`self.BP_Component_Container`)))
  (bind _returnvalue (`KismetArrayLibrary.Array_IsValidIndex` _inventory Index))
  (bind _output (`|GetArrayItem` _inventory Index))
  (if _returnvalue
    (return (and _returnvalue (> (`.Amount_9_18C02BD3F7475CFB8251C3A4A542074E` (break `/Game/WortelsGarden/Core/InventorySystem/S_InventoryItem` _output)) 0)) _output)
    (else
      (return false))))

(fn `GetIsContainerFull`
  (returns (`isFull?` :type Boolean))
  (bind _isfull_ (`/Game/WortelsGarden/Core/InventorySystem/BP_Component_Container.CheckIfInventoryFull` (`self.BP_Component_Container`)))
  (return _isfull_))

(fn `GetNameValue`
  (params (ValueName :type Name))
  (returns (ReturnValue :type Name))
  (return "None"))

(fn `GetParticipantDisplayName`
  (params (ActiveSpeaker :type Name))
  (returns (ReturnValue :type Text))
  (return (`/Game/WortelsGarden/Core/NPCs/BPC_DialogueParticipant.GetParticipantDisplayName` (`self.BPC_DialogueParticipant`) ActiveSpeaker)))

(fn `GetParticipantGender`
  (returns (ReturnValue :type "ETextGender Enum"))
  (return (`/Game/WortelsGarden/Core/NPCs/BPC_DialogueParticipant.GetParticipantGender` (`self.BPC_DialogueParticipant`))))

(fn `GetParticipantIcon`
  (params (ActiveSpeaker :type Name) (ActiveSpeakerState :type Name))
  (returns (ReturnValue :type "Texture2D Object Reference"))
  (return (`/Game/WortelsGarden/Core/NPCs/BPC_DialogueParticipant.GetParticipantIcon` (`self.BPC_DialogueParticipant`) ActiveSpeaker ActiveSpeakerState)))

(fn `GetParticipantName`
  (returns (ReturnValue :type Name))
  (return (`/Game/WortelsGarden/Core/NPCs/BPC_DialogueParticipant.GetParticipantName` (`self.BPC_DialogueParticipant`))))

(fn `GetRMB`
  (returns (`RMB?` :type Boolean))
  (return false))

(fn `GetShouldGamePause`
  (returns (`PauseGame?` :type Boolean))
  (return false))

(fn `GetTimePaused?`
  (returns (`isTimePaused?` :type Boolean))
  (return false))

(fn `GetZoomSensitivity`
  (returns (ZoomSensitivity :type "Float (double-precision)"))
  (return 0.0))

(fn `HideInteract`
  (returns (`success?` :type Boolean))
  (return false))

(fn `ModifyBoolValue`
  (params (ValueName :type Name) (bNewValue :type Boolean))
  (returns (ReturnValue :type Boolean))
  (return false))

(fn `ModifyFloatValue`
  (params (ValueName :type Name) (bDelta :type Boolean) (Value :type "Float (single-precision)"))
  (returns (ReturnValue :type Boolean))
  (return false))

(fn `ModifyIntValue`
  (params (ValueName :type Name) (bDelta :type Boolean) (Value :type Integer))
  (returns (ReturnValue :type Boolean))
  (return false))

(fn `ModifyNameValue`
  (params (ValueName :type Name) (NameValue :type Name))
  (returns (ReturnValue :type Boolean))
  (return false))

(fn `OnDialogueEvent`
  (params (Context :type "DlgContext Object Reference") (EventName :type Name))
  (returns (ReturnValue :type Boolean))
  (return false))

(fn `RemoveActiveWidget`
  (params (Widget :type "Widget Object Reference"))
  (returns (`success?` :type Boolean))
  (bind _returnvalue (`KismetArrayLibrary.Array_RemoveItem` (`self.ActiveWidgets`) Widget))
  (return _returnvalue))

(fn `RemoveEnergy`
  (params (EnergyToRemove :type "Float (double-precision)"))
  (returns (RemainingEnergy :type "Float (double-precision)"))
  (return 0.0))

(fn `RemoveFromContainer`
  (params (Name :type Name) (Variation :type Integer) (Amount :type Integer))
  (returns (`success?` :type Boolean) (AmountLeftToRemove :type Integer))
  (bind (_success_ _amountlefttoremove) (`/Game/WortelsGarden/Core/InventorySystem/BP_Component_Container.RemoveFromInventory` (`self.BP_Component_Container`) Name Variation Amount))
  (return _success_ _amountlefttoremove))

(fn `RemoveFromContainerByIndex`
  (params (Index :type Integer) (Amount :type Integer))
  (returns (AmountLeftToRemove :type Integer))
  (bind _amountlefttoremove (`/Game/WortelsGarden/Core/InventorySystem/BP_Component_Container.RemoveFromInventoryByIndex` (`self.BP_Component_Container`) Index Amount))
  (return _amountlefttoremove))

(fn `RemoveInteractable`
  (params (Actor :type "Actor Object Reference"))
  (returns (NewActiveActor :type "Actor Object Reference") (`wasActive?` :type Boolean) (`success?` :type Boolean))
  (locals (`WasActiveInteractable?` :type Boolean))
  (bind _interactables (`self.Interactables`))
  (bind _returnvalue (`KismetArrayLibrary.Array_LastIndex` _interactables))
  (message `/Game/WortelsGarden/Core/Player/BPI_Interact.HideInteract` Actor)
  (bind _output_get (set `local.WasActiveInteractable?` (== Actor (`self.ActiveInteractable`))))
  (bind _returnvalue_2 (`KismetArrayLibrary.Array_RemoveItem` _interactables Actor))
  (if _output_get
    (if (`KismetArrayLibrary.Array_IsValidIndex` _interactables _returnvalue)
      (bind _output_get_2 (set `self.ActiveInteractable` (`|GetArrayItem` _interactables _returnvalue)))
      (message `/Game/WortelsGarden/Core/Player/BPI_Interact.ShowInteract` _output_get_2)
      (return _output_get_2 (`local.WasActiveInteractable?`) _returnvalue_2)
      (else
        (set `self.ActiveInteractable` null))))
  (return (`self.ActiveInteractable`) (`local.WasActiveInteractable?`) _returnvalue_2))

(fn `SetAllClothing`
  (for (_array_element _array_index) (`|MakeArray` (`self.Clothing`) (`self.Clothing1`) (`self.Clothing2`))
    (bind _asbp_clothing (cast `/Game/WortelsGarden/Core/Player/BP_Clothing` (`ChildActorComponent.ChildActor` _array_element)))
    (bind _returnvalue (select `int` _array_index :`0` (`self.ClothingItem_0`) :`1` (`self.ClothingItem_1`) :`2` (`self.ClothingItem_2`)))
    (`SceneComponent.SetVisibility` (`/Game/WortelsGarden/Core/Player/BP_Clothing.DefaultSceneRoot` _asbp_clothing) (`|EnumInequality` _returnvalue "NewEnumerator0") true)
    (bind _returnvalue_2 (`|GetDataTableRow` "/Game/WortelsGarden/Art/Characters/Wortel/DT_ClothingItems.DT_ClothingItems" (`KismetStringLibrary.Conv_StringToName` (`|GetEnumeratorNameAsString` _returnvalue)))
      (:`then`
        (`PaperZDAnimationComponent.SetAnimInstanceClass` (`/Game/WortelsGarden/Core/Player/BP_Clothing.PaperZDAnimation` _asbp_clothing) (`.AnimationInstance_6_33E8B8C3AB43C1A33AB10BBFE0C59239` (break `/Game/WortelsGarden/Art/Characters/Wortel/S_ClothingItem` _returnvalue_2)))))))

(fn `ShowInteract`
  (returns (`success?` :type Boolean))
  (return false))

(fn `UserConstructionScript`
  (`self.SetAllClothing`))