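; BP_Camera is the camera actor that follows the player across the level within set bounds.
; Every Tick it copies the player pawn's X and Y, clamps each between MinBounds and MaxBounds, and moves itself there while keeping its own Z.
; The clamped X and Y are also printed each frame as debug output.
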(event `self.ReceiveTick`
  (params (DeltaSeconds :type "Float (single-precision)"))
  (bind (_returnvalue_x _returnvalue_y _returnvalue_z) (`KismetMathLibrary.BreakVector` (`self.K2_GetActorLocation`)))
  (bind (_minbounds_x _minbounds_y) (`KismetMathLibrary.BreakVector2D` (`self.MinBounds`)))
  (bind (_maxbounds_x _maxbounds_y) (`KismetMathLibrary.BreakVector2D` (`self.MaxBounds`)))
  (bind (_returnvalue_x_2 _returnvalue_y_2) (`KismetMathLibrary.BreakVector` (`self.K2_GetActorLocation` (`GameplayStatics.GetPlayerPawn` 0))))
  (bind _returnvalue (`KismetMathLibrary.FClamp` _returnvalue_x_2 _minbounds_x _maxbounds_x))
  (bind _returnvalue_2 (`KismetMathLibrary.FClamp` _returnvalue_y_2 _minbounds_y _maxbounds_y))
  (`self.K2_SetActorLocation` (`KismetMathLibrary.MakeVector` _returnvalue _returnvalue_2 _returnvalue_z))
  (`KismetSystemLibrary.PrintString` (`KismetStringLibrary.Concat_StrStr` "X: " (`KismetStringLibrary.Conv_DoubleToString` _returnvalue) "   Y: " (`KismetStringLibrary.Conv_DoubleToString` _returnvalue_2))))

(fn `UserConstructionScript`)