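; Blueprint for the NPC Biet, with a function that opens an item shop.
; OpenBietShop creates WBP_ItemShop for the first player, adds it to the viewport, passes itself as owning actor via a message call and opens it, printing a debug string.
; OnDialogueEvent switches on the event name with no actions attached and returns false; nothing in this graph calls OpenBietShop.
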(fn `OnDialogueEvent`
  (params (Context :type "DlgContext Object Reference") (EventName :type Name))
  (returns (ReturnValue :type Boolean))
  (`|SwitchDialogueCallbackEvent` EventName
    (:`Default`
      (return false))))

(fn `OpenBietShop`
  (bind _returnvalue (`|CreateWidget` "/Game/WortelsGarden/UI/ItemShop/WBP_ItemShop.WBP_ItemShop_C" (`GameplayStatics.GetPlayerController` 0)))
  (`UserWidget.AddToViewport` _returnvalue 0)
  (message `/Game/WortelsGarden/UI/BPI_WidgetInteract.SetOwningActor` _returnvalue self)
  (message `/Game/WortelsGarden/UI/BPI_WidgetInteract.OpenWidget` _returnvalue)
  (`KismetSystemLibrary.PrintString` "Open shop"))

(fn `UserConstructionScript`
  (`parent.UserConstructionScript`))