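; NPC character for WortelsGarden that supports dialogue, following an actor, a vendor shop and an item container.
; An overlap sphere shows a prompt and registers the NPC with the player, enabling Interact or click to start dialogue.
; Following re-issues SimpleMoveToActor on a looping, pausable timer.
; Interface functions forward to dialogue participant and container components, though dialogue value/condition functions are stubs and shop generation only stores the day.
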(event `InputAxis|MoveRight`
  (params (AxisValue :type "Float (single-precision)"))
  (`self.AddMovementInput` (`KismetMathLibrary.MakeVector` AxisValue)))

(event `InputAxis|MoveBack`
  (params (AxisValue :type "Float (single-precision)"))
  (`self.AddMovementInput` (`KismetMathLibrary.MakeVector` 0.0 AxisValue)))

(event `self.DialogueSphere.OnComponentBeginOverlap`
  (params (OverlappedComponent :type "PrimitiveComponent Object Reference") (OtherActor :type "Actor Object Reference") (OtherComp :type "PrimitiveComponent Object Reference") (OtherBodyIndex :type Integer) (bFromSweep :type Boolean) (SweepResult :type "HitResult Structure (by ref)"))
  (if (== OtherActor (`GameplayStatics.GetPlayerPawn` 0))
    (if (and (`self.canHaveDialogue?`) (not (`self.inDialogue?`)))
      (`SceneComponent.SetVisibility` (`self.DlgPrompt`) true false)
      (set `self.inDialogueRange?` true)
      (message `/Game/WortelsGarden/Core/Player/BPI_Interact.AddInteractable` (`GameplayStatics.GetPlayerPawn` 0) self true))))

(event `self.DialogueSphere.OnComponentEndOverlap`
  (params (OverlappedComponent :type "PrimitiveComponent Object Reference") (OtherActor :type "Actor Object Reference") (OtherComp :type "PrimitiveComponent Object Reference") (OtherBodyIndex :type Integer))
  (if (== OtherActor (`GameplayStatics.GetPlayerPawn` 0))
    (`SceneComponent.SetVisibility` (`self.DlgPrompt`) false false)
    (set `self.inDialogueRange?` false)
    (message `/Game/WortelsGarden/Core/Player/BPI_Interact.RemoveInteractable` (`GameplayStatics.GetPlayerPawn` 0) self)))

(event `/Game/WortelsGarden/Core/Player/BPI_Interact.Interact`
  (if (and (`self.canHaveDialogue?`) (`self.inDialogueRange?`) (not (`self.inDialogue?`))) :!label _label
    (message `/Game/WortelsGarden/UI/Dialogue/BPI_Dialogue.StartDialogueWithNPC` (`GameplayStatics.GetPlayerPawn` 0) (`/Game/WortelsGarden/Core/NPCs/BPC_DialogueParticipant.Dialogue` (`self.BPC_DialogueParticipant`)) self)
    (bind _returnvalue (`|CreateWidget` "/Game/WortelsGarden/UI/Dialogue/WBP_Dialogue.WBP_Dialogue_C" (`GameplayStatics.GetPlayerController` 0)))
    (`UserWidget.AddToViewport` _returnvalue 1)
    (message `/Game/WortelsGarden/UI/Dialogue/BPI_Dialogue.SetDialogueWidget` (`GameplayStatics.GetPlayerPawn` 0) _returnvalue)
    (`self.SetInDialogue` true)
    (message `/Game/WortelsGarden/UI/BPI_WidgetInteract.OpenWidget` _returnvalue)
    (elif (`self.inDialogue?`)
      (message `/Game/WortelsGarden/UI/Dialogue/BPI_Dialogue.GetDialogueWidget` (`GameplayStatics.GetPlayerPawn` 0)))))

(event `self.ClickBox.OnClicked`
  (params (TouchedComponent :type "PrimitiveComponent Object Reference") (ButtonPressed :type "Key Structure"))
  (`KismetSystemLibrary.PrintString` "click NPC")
  (goto _label))

(event `/Game/WortelsGarden/UI/Dialogue/BPI_Dialogue.SetInDialogue`
  (params (`inDialogue?` :type Boolean))
  (bind _output_get (set `self.inDialogue?` `inDialogue?`))
  (`SceneComponent.SetVisibility` (`self.DlgPrompt`) (and (not _output_get) (`self.inDialogueRange?`)) false))

(event `/Game/WortelsGarden/Core/InventorySystem/BPI_InventorySystem.UpdateContainer`
  (params (IndexToUpdate :type Integer) (`UpdateAllIndexes?` :type Boolean))
  (message `/Game/WortelsGarden/Core/InventorySystem/BPI_InventorySystem.UpdateContainer` (`self.BP_Component_Container`) IndexToUpdate `UpdateAllIndexes?`))

(fn `AddInteractable`
  (params (Actor :type "Actor Object Reference") (`SetActive?` :type Boolean))
  (returns (`success?` :type Boolean))
  (return false))

(fn `AddToContainer`
  (params (Item :type "/Game/WortelsGarden/Core/InventorySystem/S_InventoryItem Structure"))
  (returns (`success?` :type Boolean) (Index :type Integer))
  (bind (_success_ _index) (`/Game/WortelsGarden/Core/InventorySystem/BP_Component_Container.AddToInventory` (`self.BP_Component_Container`) Item))
  (return _success_ _index))

(fn `AddToContainerByIndex`
  (params (Item :type "/Game/WortelsGarden/Core/InventorySystem/S_InventoryItem Structure") (Index :type Integer))
  (returns (`success?` :type Boolean))
  (bind _success_ (`/Game/WortelsGarden/Core/InventorySystem/BP_Component_Container.AddToInventoryByIndex` (`self.BP_Component_Container`) Item Index))
  (return _success_))

(fn `CheckCondition`
  (params (Context :type "DlgContext Object Reference") (ConditionName :type Name))
  (returns (ReturnValue :type Boolean))
  (return false))

(fn `FindEmptyIndex`
  (returns (`foundIndex?` :type Boolean) (Index :type Integer))
  (bind (_foundindex_ _index) (`/Game/WortelsGarden/Core/InventorySystem/BP_Component_Container.FindEmptyIndex` (`self.BP_Component_Container`)))
  (return _foundindex_ _index))

(fn `FindInContaineer`
  (return))

(fn `FindInContainer`
  (params (Name :type Name) (Variation :type Integer))
  (returns (`isFound?` :type Boolean) (ItemIndex :type Integer))
  (bind (_isfound_ _itemindex) (`/Game/WortelsGarden/Core/InventorySystem/BP_Component_Container.FindInInventory` (`self.BP_Component_Container`) Name Variation))
  (return _isfound_ _itemindex))

(fn `FollowActor`
  (params (FollowActor :type "Actor Object Reference"))
  (set `self.FollowingActor` FollowActor)
  (if (`KismetSystemLibrary.K2_IsTimerActive` null "FollowActorTimer")
    _
    (elif (`KismetSystemLibrary.K2_IsTimerPaused` null "FollowActorTimer")
      (`KismetSystemLibrary.K2_UnPauseTimer` null "FollowActorTimer")
      (else
        (`KismetSystemLibrary.K2_SetTimer` null "FollowActorTimer" 0.1 true)))))

(fn `FollowActorTimer`
  (bind _followingactor (`self.FollowingActor`)
    (:`then`
      (`AIBlueprintHelperLibrary.SimpleMoveToActor` (`self.GetController`) _followingactor))
    (:`else`
      (`KismetSystemLibrary.PrintString` "follow actor not valid, aborting follow")
      (`self.StopFollowingActor` null))))

(fn `GenerateShopInventory`
  (params (Day :type Integer))
  (set `self.ShopDay` Day))

(fn `GetBoolValue`
  (params (ValueName :type Name))
  (returns (ReturnValue :type Boolean))
  (return false))

(fn `GetContainer`
  (returns (Container :type "/Game/WortelsGarden/Core/InventorySystem/BP_Component_Container Object Reference"))
  (return (`self.BP_Component_Container`)))

(fn `GetDialogueContext`
  (returns (DialogueContext :type "DlgContext Object Reference"))
  (return null))

(fn `GetDialogueWidget`
  (returns (DialogueWidget :type "Widget Object Reference"))
  (return null))

(fn `GetFloatValue`
  (params (ValueName :type Name))
  (returns (ReturnValue :type "Float (single-precision)"))
  (return 0.0))

(fn `GetFollowActor`
  (returns (FollowActor :type "Actor Object Reference") (FollowOffset :type "Vector Structure"))
  (return (`self.FollowingActor`) (`self.FollowingOffset`)))

(fn `GetInDialgoue`
  (returns (`inDialogue?` :type Boolean))
  (return (`self.inDialogue?`)))

(fn `GetInteractable`
  (returns (ActiveInteractable :type "Actor Object Reference") (Interactables :type "Array of Actor Object Reference"))
  (return null))

(fn `GetIntValue`
  (params (ValueName :type Name))
  (returns (ReturnValue :type Integer))
  (return 0))

(fn `GetInventory`
  (returns (Inventory :type "Array of /Game/WortelsGarden/Core/InventorySystem/S_InventoryItem Structure"))
  (return (`/Game/WortelsGarden/Core/InventorySystem/BP_Component_Container.Inventory` (`self.BP_Component_Container`))))

(fn `GetInventoryItemByIndex`
  (params (Index :type Integer))
  (returns (`hasItem?` :type Boolean) (InventoryItem :type "/Game/WortelsGarden/Core/InventorySystem/S_InventoryItem Structure"))
  (bind (_hasitem_ _inventoryitem) (message `/Game/WortelsGarden/Core/InventorySystem/BPI_InventorySystem.GetInventoryItemByIndex` (`self.BP_Component_Container`) Index))
  (return _hasitem_ _inventoryitem))

(fn `GetIsContainerFull`
  (returns (`isFull?` :type Boolean))
  (bind _isfull_ (`/Game/WortelsGarden/Core/InventorySystem/BP_Component_Container.CheckIfInventoryFull` (`self.BP_Component_Container`)))
  (return _isfull_))

(fn `GetIsFollowingActor?`
  (returns (`isFollowingActor?` :type Boolean))
  (return (`KismetSystemLibrary.IsValid` (`self.FollowingActor`))))

(fn `GetNameValue`
  (params (ValueName :type Name))
  (returns (ReturnValue :type Name))
  (return "None"))

(fn `GetParticipantDisplayName`
  (params (ActiveSpeaker :type Name))
  (returns (ReturnValue :type Text))
  (return (`/Game/WortelsGarden/Core/NPCs/BPC_DialogueParticipant.GetParticipantDisplayName` (`self.BPC_DialogueParticipant`) ActiveSpeaker)))

(fn `GetParticipantGender`
  (returns (ReturnValue :type "ETextGender Enum"))
  (return (`/Game/WortelsGarden/Core/NPCs/BPC_DialogueParticipant.GetParticipantGender` (`self.BPC_DialogueParticipant`))))

(fn `GetParticipantIcon`
  (params (ActiveSpeaker :type Name) (ActiveSpeakerState :type Name))
  (returns (ReturnValue :type "Texture2D Object Reference"))
  (return (`/Game/WortelsGarden/Core/NPCs/BPC_DialogueParticipant.GetParticipantIcon` (`self.BPC_DialogueParticipant`) ActiveSpeaker ActiveSpeakerState)))

(fn `GetParticipantName`
  (returns (ReturnValue :type Name))
  (return (`/Game/WortelsGarden/Core/NPCs/BPC_DialogueParticipant.GetParticipantName` (`self.BPC_DialogueParticipant`))))

(fn `GetVendorInfo`
  (returns (`success?` :type Boolean) (VendorPortrait :type "Texture2D Object Reference") (VendorDisplayName :type Text) (VendorBarks :type "Array of Text"))
  (return true (`self.VendorPortrait`) (`/Game/WortelsGarden/Core/NPCs/BPC_DialogueParticipant.DisplayName` (`self.BPC_DialogueParticipant`)) (`self.VendorBarks`)))

(fn `HideInteract`
  (returns (`success?` :type Boolean))
  (return false))

(fn `ModifyBoolValue`
  (params (ValueName :type Name) (bNewValue :type Boolean))
  (returns (ReturnValue :type Boolean))
  (return false))

(fn `ModifyFloatValue`
  (params (ValueName :type Name) (bDelta :type Boolean) (Value :type "Float (single-precision)"))
  (returns (ReturnValue :type Boolean))
  (return false))

(fn `ModifyIntValue`
  (params (ValueName :type Name) (bDelta :type Boolean) (Value :type Integer))
  (returns (ReturnValue :type Boolean))
  (return false))

(fn `ModifyNameValue`
  (params (ValueName :type Name) (NameValue :type Name))
  (returns (ReturnValue :type Boolean))
  (return false))

(fn `OnDialogueEvent`
  (params (Context :type "DlgContext Object Reference") (EventName :type Name))
  (returns (ReturnValue :type Boolean))
  (`|SwitchDialogueCallbackEvent` EventName
    (:`Default`
      (return false))))

(fn `OpenShop`
  (bind _returnvalue (`|CreateWidget` (`self.ShopWidget`) (`GameplayStatics.GetPlayerController` 0)))
  (`UserWidget.AddToViewport` _returnvalue 0)
  (message `/Game/WortelsGarden/UI/BPI_WidgetInteract.SetOwningActor` _returnvalue self)
  (message `/Game/WortelsGarden/UI/BPI_WidgetInteract.OpenWidget` _returnvalue)
  (`KismetSystemLibrary.PrintString` "Open shop"))

(fn `RemoveFromContainer`
  (params (Name :type Name) (Variation :type Integer) (Amount :type Integer))
  (returns (`success?` :type Boolean) (AmountLeftToRemove :type Integer))
  (bind (_success_ _amountlefttoremove) (`/Game/WortelsGarden/Core/InventorySystem/BP_Component_Container.RemoveFromInventory` (`self.BP_Component_Container`) Name Variation Amount))
  (return _success_ _amountlefttoremove))

(fn `RemoveFromContainerByIndex`
  (params (Index :type Integer) (Amount :type Integer))
  (returns (AmountLeftToRemove :type Integer))
  (bind _amountlefttoremove (`/Game/WortelsGarden/Core/InventorySystem/BP_Component_Container.RemoveFromInventoryByIndex` (`self.BP_Component_Container`) Index Amount))
  (return _amountlefttoremove))

(fn `RemoveInteractable`
  (params (Actor :type "Actor Object Reference")))

(fn `SetWalkSpeed`
  (params (Multiplier :type "Float (double-precision)"))
  (set `CharacterMovementComponent.MaxWalkSpeed` (* Multiplier (`self.DefaultWalkSpeed`)) (`self.CharacterMovement`)))

(fn `ShowInteract`
  (returns (`success?` :type Boolean))
  (return false))

(fn `StopFollowingActor`
  (params (FollowActor :type "Actor Object Reference"))
  (returns (`success?` :type Boolean))
  (`/Engine/EditorBlueprintResources/StandardMacros.IsValid` FollowActor
    (:`Is Valid`
      (if (== FollowActor (`self.FollowingActor`))
        _
        (else
          (`KismetSystemLibrary.PrintString` "follow actor does not match")
          (return false))))
    (:`Is Not Valid`
      _))
  (set `self.FollowingActor` null)
  (`KismetSystemLibrary.K2_PauseTimer` null "FollowActorTimer")
  (return true))

(fn `UserConstructionScript`
  (bind _widget (`self.Widget`))
  (bind (_relativelocation_x _relativelocation_y _relativelocation_z) (`KismetMathLibrary.BreakVector` (`SceneComponent.RelativeLocation` _widget)))
  (`|ExecutionSequence`
    (:`then_0`
      (`SceneComponent.K2_SetRelativeLocation` _widget (`KismetMathLibrary.MakeVector` _relativelocation_x (`self.DialogueOffset`) _relativelocation_z) false false)
      (`SphereComponent.SetSphereRadius` (`self.DialogueSphere`) (`self.DialogueRange`) true))
    (:`then_1`
      (`self.SetWalkSpeed` 1.0))))