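; Placeable, rotatable bed sprite that lets the player sleep to regain energy.
; Rotation and variation select the foreground sprite, and rotation parity decides which of two overlap volumes is active.
; Player or NPC overlap, unless picked up, reveals the foreground and starts a looping Rest timer raising player energy toward a cap.
; It also sets the player's sleep animation and delayed emote, even for NPC overlaps; end overlap reverses this.
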(event `self.ShowFG.OnComponentBeginOverlap`
  (params (OverlappedComponent :type "PrimitiveComponent Object Reference") (OtherActor :type "Actor Object Reference") (OtherComp :type "PrimitiveComponent Object Reference") (OtherBodyIndex :type Integer) (bFromSweep :type Boolean) (SweepResult :type "HitResult Structure (by ref)"))
  (if (and (not (`self.isPickedUp?`)) (or (== (`GameplayStatics.GetPlayerPawn` 0) OtherActor) (== (`GameplayStatics.GetObjectClass` OtherActor) "/Game/WortelsGarden/Core/NPCs/BP_NPC.BP_NPC_C")) (not (> (mod (`self.Rotation`) 2) 0)))
    (`SceneComponent.SetHiddenInGame` (`self.SpriteFG`) false false)
    (`KismetSystemLibrary.PrintString` "show FG")
    (if (not (`KismetSystemLibrary.K2_TimerExists` null "Rest")) :!label _label
      (`KismetSystemLibrary.K2_SetTimer` null "Rest" 0.1 true)
      (bind _asbp_wortel (cast `/Game/WortelsGarden/Core/Player/BP_Wortel` (`GameplayStatics.GetPlayerPawn` 0)))
      (bind _asabp_wortel (cast `/Game/WortelsGarden/Art/Characters/Wortel/ABP_Wortel` (`PaperZDCharacter.GetAnimInstance` _asbp_wortel)))
      (set `/Game/WortelsGarden/Art/Characters/Wortel/ABP_Wortel.isSleeping?` true _asabp_wortel)
      (`KismetSystemLibrary.RetriggerableDelay` 0.5)
      (if (`KismetSystemLibrary.K2_TimerExists` null "Rest")
        (`SceneComponent.SetVisibility` (`/Game/WortelsGarden/Core/Player/BP_Wortel.Emote` _asbp_wortel) true false)))))

(event `self.ShowFG.OnComponentEndOverlap`
  (params (OverlappedComponent :type "PrimitiveComponent Object Reference") (OtherActor :type "Actor Object Reference") (OtherComp :type "PrimitiveComponent Object Reference") (OtherBodyIndex :type Integer))
  (if (not (> (mod (`self.Rotation`) 2) 0))
    (`SceneComponent.SetHiddenInGame` (`self.SpriteFG`) true false)
    (`KismetSystemLibrary.PrintString` "hide FG")
    (`KismetSystemLibrary.K2_ClearTimer` null "Rest" :!label _label_2)
    (bind _asbp_wortel (cast `/Game/WortelsGarden/Core/Player/BP_Wortel` (`GameplayStatics.GetPlayerPawn` 0)))
    (bind _asabp_wortel (cast `/Game/WortelsGarden/Art/Characters/Wortel/ABP_Wortel` (`PaperZDCharacter.GetAnimInstance` _asbp_wortel)))
    (set `/Game/WortelsGarden/Art/Characters/Wortel/ABP_Wortel.isSleeping?` false _asabp_wortel)
    (bind _energy (message `/Game/WortelsGarden/Core/Player/BPI_PlayerData.GetEnergy` (`GameplayStatics.GetPlayerController` 0)))
    (if (not (< _energy 1.0))
      (`SceneComponent.SetVisibility` (`/Game/WortelsGarden/Core/Player/BP_Wortel.Emote` _asbp_wortel) false false))))

(event `self.RotatedShowFG.OnComponentBeginOverlap`
  (params (OverlappedComponent :type "PrimitiveComponent Object Reference") (OtherActor :type "Actor Object Reference") (OtherComp :type "PrimitiveComponent Object Reference") (OtherBodyIndex :type Integer) (bFromSweep :type Boolean) (SweepResult :type "HitResult Structure (by ref)"))
  (if (and (not (`self.isPickedUp?`)) (or (== (`GameplayStatics.GetPlayerPawn` 0) OtherActor) (== (`GameplayStatics.GetObjectClass` OtherActor) "/Game/WortelsGarden/Core/NPCs/BP_NPC.BP_NPC_C")) (> (mod (`self.Rotation`) 2) 0))
    (`SceneComponent.SetHiddenInGame` (`self.SpriteFG`) false false)
    (goto _label)))

(event `self.RotatedShowFG.OnComponentEndOverlap`
  (params (OverlappedComponent :type "PrimitiveComponent Object Reference") (OtherActor :type "Actor Object Reference") (OtherComp :type "PrimitiveComponent Object Reference") (OtherBodyIndex :type Integer))
  (if (> (mod (`self.Rotation`) 2) 0)
    (`SceneComponent.SetHiddenInGame` (`self.SpriteFG`) true false)
    (goto _label_2)))

(event `/Game/WortelsGarden/Core/Sprites/BPI_Grid.Rotate`
  (`parent.Rotate`)
  (`self.SetFGSprite`)
  (`self.SetCollision`))

(event `/Game/WortelsGarden/Core/Sprites/BPI_SpriteActions.SetVariation`
  (params (Variation :type Integer))
  (set `self.Variation` Variation)
  (`self.SetSprite`)
  (`self.SetFGSprite`))

(fn `Rest`
  (bind _asbp_player_controller (cast `/Game/WortelsGarden/Core/Player/BP_PlayerController` (`GameplayStatics.GetPlayerController` 0)))
  (bind _energy (`/Game/WortelsGarden/Core/Player/BP_PlayerController.Energy` _asbp_player_controller))
  (if (< _energy 10.0)
    (set `/Game/WortelsGarden/Core/Player/BP_PlayerController.Energy` (+ _energy 0.03) _asbp_player_controller)))

(fn `SetFGSprite`
  (bind _fgvariationsprites (`self.FGVariationSprites`))
  (bind _variation (`self.Variation`))
  (bind (_output_top _output_right _output_bottom _output_left) (break `/Game/WortelsGarden/Core/Sprites/S_SpriteVariation` (`|GetArrayItem` _fgvariationsprites _variation)))
  (if (`KismetArrayLibrary.Array_IsValidIndex` _fgvariationsprites _variation)
    (`PaperSpriteComponent.SetSprite` (`self.SpriteFG`) (select `int` (`self.Rotation`) :`0` _output_top :`1` _output_right :`2` _output_bottom :`3` _output_left))
    (`self.SetOverlapResponses`)))

(fn `SetOverlapResponses`
  (bind _returnvalue (> (mod (`self.Rotation`) 2) 0))
  (set `PrimitiveComponent.bGenerateOverlapEvents` (not _returnvalue) (`self.ShowFG`))
  (set `PrimitiveComponent.bGenerateOverlapEvents` _returnvalue (`self.RotatedShowFG`)))

(fn `UserConstructionScript`
  (`parent.UserConstructionScript`)
  (`|ExecutionSequence`
    (:`then_0`
      ;[0.01891 0.01891 0.01891] Foreground Sprite
      (`self.SetFGSprite`))))