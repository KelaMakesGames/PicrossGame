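; Placeable grid fence sprite that auto-tiles to connect with neighbouring fences of the same class.
; Four vertical line traces, one per orthogonal neighbour tile, set the Has*Fence flags, which are matched against 16 patterns to choose the Variation.
; A changed Variation swaps the sprite and enables box collision only on connected sides.
; It refreshes on construction, BeginPlay, in-range grid clicks and placability updates, which also message surrounding fences to update.
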(event `self.ReceiveBeginPlay`
  (`parent.ReceiveBeginPlay`)
  (`self.UpdateFenceVariation` false))

(event `self.Grid.OnClicked`
  (params (TouchedComponent :type "PrimitiveComponent Object Reference") (ButtonPressed :type "Key Structure"))
  (if (`self.inGridInteractableRange?`)
    (`self.FindSurroundingFences` false)
    (`self.SetTileType`)))

(event `/Game/WortelsGarden/Core/Sprites/BPI_AutoTile.UpdateSurroundingTiles`
  (params (`FindSurroundingFencesFirst?` :type Boolean))
  (if `FindSurroundingFencesFirst?`
    (`self.FindSurroundingFences` false))
  (for _array_element (`self.SurroundingFences`)
    (message `/Game/WortelsGarden/Core/Sprites/BPI_AutoTile.UpdateTile` _array_element)))

(event `/Game/WortelsGarden/Core/Sprites/BPI_AutoTile.UpdateTile`
  (`self.UpdateFenceVariation` false))

(event `/Game/WortelsGarden/Core/Sprites/BPI_Grid.UpdatePlacability`
  (`parent.UpdatePlacability`)
  (`self.UpdateSurroundingTiles` false)
  (`self.UpdateSurroundingTiles` true)
  (`self.UpdateFenceVariation` false))

(fn `FindSurroundingFences`
  (params (`Debug?` :type Boolean))
  (bind (_returnvalue_x _returnvalue_y) (`KismetMathLibrary.BreakVector` (`self.K2_GetActorLocation`)))
  (`KismetArrayLibrary.Array_Clear` (`self.SurroundingFences`))
  (set `self.hasTopFence?` false)
  (set `self.hasRightFence?` false)
  (set `self.hasBottomFence?` false)
  (set `self.hasLeftFence?` false)
  (for _index (range 4)
    (bind _returnvalue (- (+ _returnvalue_x (select `int` _index :`0` 0.0 :`1` 50.0 :`2` 0.0 :`3` -50.0)) 25.0))
    (bind _returnvalue_2 (- (+ _returnvalue_y (select `int` _index :`0` -50.0 :`1` 0.0 :`2` 50.0 :`3` 0.0)) 25.0))
    (bind (_outhit _returnvalue_3) (`KismetSystemLibrary.LineTraceSingle` :`Start` (`KismetMathLibrary.MakeVector` _returnvalue _returnvalue_2 100.0) :`End` (`KismetMathLibrary.MakeVector` _returnvalue _returnvalue_2 -100.0) :`TraceChannel` "TraceTypeQuery4" :`DrawDebugType` "ForDuration" :`TraceColor` (struct :`R` 1.0 :`G` 1.0 :`B` 1.0 :`A` 1.0) :`DrawTime` 2.0))
    (if _returnvalue_3
      (bind (_bblockinghit _binitialoverlap _time _distance _location _impactpoint _normal _impactnormal _physmat _hitactor) (`GameplayStatics.BreakHitResult` _outhit))
      (if (== (`GameplayStatics.GetObjectClass` _hitactor) (`GameplayStatics.GetObjectClass` self))
        (`KismetArrayLibrary.Array_Set` (`self.SurroundingFences`) _index _hitactor true)
        (if `Debug?`
          (message `/Game/WortelsGarden/Core/Sprites/BPI_Grid.FlashGrid` _hitactor))
        (switch `int` _index
          (:`0`
            (set `self.hasTopFence?` true))
          (:`1`
            (set `self.hasRightFence?` true))
          (:`2`
            (set `self.hasBottomFence?` true))
          (:`3`
            (set `self.hasLeftFence?` true)))))))

(fn `GetTileVariation`
  (returns (Variation :type Integer))
  (return (`self.Variation`)))

(fn `SetAllBoxCollisions`
  (params (`showCollisions?` :type Boolean))
  (bind _variation (`self.Variation`))
  (`|ExecutionSequence`
    (:`then_0`
      (bind _output_get (set `self.LeftCollision?` (select `int` _variation :`0` false :`1` false :`2` true :`3` true :`4` false :`5` false :`6` true :`7` true :`8` false :`9` false :`10` true :`11` true :`12` false :`13` false :`14` true :`15` true :`16` false)))
      (`self.SetBoxCollision` _output_get (`self.Box_Left`)))
    (:`then_1`
      (bind _output_get_2 (set `self.RightCollision?` (select `int` _variation :`0` false :`1` true :`2` true :`3` false :`4` false :`5` true :`6` true :`7` false :`8` false :`9` true :`10` true :`11` false :`12` false :`13` true :`14` true :`15` false :`16` false)))
      (`self.SetBoxCollision` _output_get_2 (`self.Box_Right`)))
    (:`then_2`
      (bind _output_get_3 (set `self.BottomCollision?` (select `int` _variation :`0` true :`1` true :`2` true :`3` true :`4` true :`5` true :`6` true :`7` true :`8` false :`9` false :`10` false :`11` false :`12` false :`13` false :`14` false :`15` false :`16` false)))
      (`self.SetBoxCollision` _output_get_3 (`self.Box_Rottom`)))
    (:`then_3`
      (bind _output_get_4 (set `self.TopCollision?` (select `int` _variation :`0` false :`1` false :`2` false :`3` false :`4` true :`5` true :`6` true :`7` true :`8` true :`9` true :`10` true :`11` true :`12` false :`13` false :`14` false :`15` false :`16` false)))
      (`self.SetBoxCollision` _output_get_4 (`self.Box_Top`)))
    (:`then_4`
      (bind _pickedupactor (message `/Game/WortelsGarden/Core/Sprites/BPI_Grid.GetPickedUpActor` (`GameplayStatics.GetPlayerController` 0)))
      (if (== _pickedupactor self)
        (`KismetSystemLibrary.PrintString` (`KismetStringLibrary.Concat_StrStr` "TOP: " (`KismetStringLibrary.Conv_BoolToString` (`self.TopCollision?`)) "  RIGHT: " (`KismetStringLibrary.Conv_BoolToString` (`self.RightCollision?`)) "  BOTTOM: " (`KismetStringLibrary.Conv_BoolToString` (`self.BottomCollision?`)) "  LEFT: " (`KismetStringLibrary.Conv_BoolToString` (`self.LeftCollision?`))) true true (struct :`G` 0.66 :`B` 1.0 :`A` 1.0) 5.0)))
    (:`then_5`
      (if `showCollisions?`
        (for (_array_element _array_index) (`|MakeArray` (`self.Box_Top`) (`self.Box_Right`) (`self.Box_Rottom`) (`self.Box_Left`))
          (`SceneComponent.SetHiddenInGame` _array_element (not (select `int` _array_index :`0` (`self.TopCollision?`) :`1` (`self.RightCollision?`) :`2` (`self.BottomCollision?`) :`3` (`self.LeftCollision?`))) false))))))

(fn `SetBoxCollision`
  (params (`CollisionEnabled?` :type Boolean) (Box :type "BoxComponent Object Reference"))
  (`PrimitiveComponent.SetCollisionEnabled` Box (select `bool` `CollisionEnabled?` :`false` "NoCollision" :`true` "QueryAndPhysics" :!type "ECollisionEnabled Enum"))
  (`PrimitiveComponent.SetCollisionResponseToChannel` Box "ECC_Pawn" (select `bool` `CollisionEnabled?` :`false` "ECR_Ignore" :`true` "ECR_Block" :!type "ECollisionResponse Enum")))

(fn `SetTileType`
  (for _index (range 16)
    (if (`KismetArrayLibrary.Array_Identical` (`|MakeArray` (`self.hasTopFence?`) (`self.hasRightFence?`) (`self.hasBottomFence?`) (`self.hasLeftFence?`)) (select `int` _index :`0` (`|MakeArray` false false true false) :`1` (`|MakeArray` false true true false) :`2` (`|MakeArray` false true true true) :`3` (`|MakeArray` false false true true) :`4` (`|MakeArray` true false true false) :`5` (`|MakeArray` true true true false) :`6` (`|MakeArray` true true true true) :`7` (`|MakeArray` true false true true) :`8` (`|MakeArray` true false false false) :`9` (`|MakeArray` true true false false) :`10` (`|MakeArray` true true false true) :`11` (`|MakeArray` true false false true) :`12` (`|MakeArray` false false false false) :`13` (`|MakeArray` false true false false) :`14` (`|MakeArray` false true false true) :`15` (`|MakeArray` false false false true)))
      (if (!= (`self.Variation`) _index)
        (bind _output_get (set `self.Variation` _index))
        (bind _output_top (break `/Game/WortelsGarden/Core/Sprites/S_SpriteVariation` (`|GetArrayItem` (`self.VariationSprites`) _output_get)))
        (`PaperSpriteComponent.SetSprite` (`self.Sprite`) _output_top)
        (`self.SetAllBoxCollisions` false)
        (break)))))

(fn `UpdateFenceVariation`
  (params (`Debug?` :type Boolean))
  (`self.FindSurroundingFences` `Debug?`)
  (`self.SetTileType`))

(fn `UserConstructionScript`
  (`parent.UserConstructionScript`)
  ;[0.01891 0.01891 0.01891] Box Collisions
  (`self.SetAllBoxCollisions` false)
  (`self.UpdateFenceVariation` false))