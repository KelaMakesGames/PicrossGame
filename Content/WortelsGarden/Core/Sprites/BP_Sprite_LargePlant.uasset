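; Large plant sprite actor for the garden grid that grows, shows its growth progress and can be harvested by clicking.
; BPComponentGrowth drives the state: grid clicks start harvest or resume growth, and picking the plant up pauses growth.
; Player overlap with GrowthTimer toggles the radial progress widget and its updates.
; A ripe plant's sprite shifts as a hover cue when in range, subject to input mode and no carried actor.
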(event `self.ReceiveBeginPlay`
  (`parent.ReceiveBeginPlay`)
  (bind _aswbp_growth_progress (cast `/Game/WortelsGarden/UI/WBP_GrowthProgress` (`WidgetComponent.GetUserWidgetObject` (`self.RadialGrowth`))))
  (set `/Game/WortelsGarden/UI/WBP_GrowthProgress.OwningPlant` self _aswbp_growth_progress))

(event `/Game/WortelsGarden/Core/Sprites/BPI_Growth.ToggleCrop`
  (params (`hasCrop?` :type Boolean))
  (`self.Toggle Crop` `hasCrop?`))

(event `/Game/WortelsGarden/Core/Sprites/BPI_Grid.SetInGridInteractableRange`
  (params (`inRange?` :type Boolean))
  (bind _output_get (set `self.inGridInteractableRange?` `inRange?`))
  (if _output_get
    (`self.ShowHarvestability`)
    (else
      (`self.HideHarvestability`))))

(event `/Game/WortelsGarden/Core/Sprites/BPI_Growth.SetReadyToBeHarvestable`
  (`self.ShowHarvestability`)
  (`KismetSystemLibrary.PrintString` (`KismetStringLibrary.Concat_StrStr` (`KismetSystemLibrary.GetDisplayName` self) " ready to be harvested")))

(event `ShowHarvestability`
  (bind _returnvalue (`GameplayStatics.GetPlayerController` 0))
  (bind _inputmode (message `/Game/WortelsGarden/Core/Player/BPI_PlayerData.GetInputMode` _returnvalue :!label _label))
  (bind (_pickedupactor _isvalidactor_) (message `/Game/WortelsGarden/Core/Sprites/BPI_Grid.GetPickedUpActor` _returnvalue))
  (`self.ShowGrid` false)
  (if (and (`|EnumEquality` _inputmode "NewEnumerator0") (`/Game/WortelsGarden/Core/Sprites/BP_Component_Growth.isReadyToBeHarvested?` (`self.BP_Component_Growth`)) (`self.isCursorOverGrid?`) (`self.inGridInteractableRange?`) (not _isvalidactor_))
    (`SceneComponent.K2_SetRelativeLocation` (`self.Sprite`) (+ (`self.DefaultRelativeLocation`) (`self.HarvestSpriteOffset`)) false false)))

(event `self.Grid.OnBeginCursorOver`
  (params (TouchedComponent :type "PrimitiveComponent Object Reference"))
  (set `self.isCursorOverGrid?` true)
  (goto _label))

(event `HideHarvestability`
  (`SceneComponent.K2_SetRelativeLocation` (`self.Sprite`) (`self.DefaultRelativeLocation`) false false :!label _label_2))

(event `self.Grid.OnEndCursorOver`
  (params (TouchedComponent :type "PrimitiveComponent Object Reference"))
  (set `self.isCursorOverGrid?` false)
  (goto _label_2))

(event `self.Grid.OnClicked`
  (params (TouchedComponent :type "PrimitiveComponent Object Reference") (ButtonPressed :type "Key Structure"))
  (bind _bp_component_growth (`self.BP_Component_Growth`))
  (message `/Game/WortelsGarden/Core/Sprites/BPI_Grid.Click` self ButtonPressed)
  (if (`/Game/WortelsGarden/Core/Sprites/BP_Component_Growth.isReadyToBeHarvested?` _bp_component_growth)
    (`/Game/WortelsGarden/Core/Sprites/BP_Component_Growth.StartHarvest` _bp_component_growth)
    (else
      (`/Game/WortelsGarden/Core/Sprites/BP_Component_Growth.ResumeGrowth` (`self.BP_Component_Growth`)))))

(event `self.GrowthTimer.OnComponentBeginOverlap`
  (params (OverlappedComponent :type "PrimitiveComponent Object Reference") (OtherActor :type "Actor Object Reference") (OtherComp :type "PrimitiveComponent Object Reference") (OtherBodyIndex :type Integer) (bFromSweep :type Boolean) (SweepResult :type "HitResult Structure (by ref)"))
  (bind _bp_component_growth (`self.BP_Component_Growth`))
  (bind _bp_component_growth_2 (`self.BP_Component_Growth`))
  (if (and (== OtherActor (`GameplayStatics.GetPlayerPawn` 0)) (or (`/Game/WortelsGarden/Core/Sprites/BP_Component_Growth.isReadyToBeHarvested?` _bp_component_growth_2) (`/Game/WortelsGarden/Core/Sprites/BP_Component_Growth.shouldGrow?` _bp_component_growth_2)))
    (`SceneComponent.SetVisibility` (`self.RadialGrowth`) (not (`self.isPickedUp?`)) false)
    (`/Game/WortelsGarden/Core/Sprites/BP_Component_Growth.ResumeUpdateShowProgress` _bp_component_growth)
    (set `/Game/WortelsGarden/Core/Sprites/BP_Component_Growth.isGrowthProgressShown?` true _bp_component_growth)))

(event `self.GrowthTimer.OnComponentEndOverlap`
  (params (OverlappedComponent :type "PrimitiveComponent Object Reference") (OtherActor :type "Actor Object Reference") (OtherComp :type "PrimitiveComponent Object Reference") (OtherBodyIndex :type Integer))
  (bind _bp_component_growth (`self.BP_Component_Growth`))
  (bind _bp_component_growth_2 (`self.BP_Component_Growth`))
  (if (and (== OtherActor (`GameplayStatics.GetPlayerPawn` 0)) (or (`/Game/WortelsGarden/Core/Sprites/BP_Component_Growth.isReadyToBeHarvested?` _bp_component_growth_2) (`/Game/WortelsGarden/Core/Sprites/BP_Component_Growth.shouldGrow?` _bp_component_growth_2)))
    (`SceneComponent.SetVisibility` (`self.RadialGrowth`) false false)
    (`/Game/WortelsGarden/Core/Sprites/BP_Component_Growth.PauseUpdateShowProgress` _bp_component_growth)
    (set `/Game/WortelsGarden/Core/Sprites/BP_Component_Growth.isGrowthProgressShown?` false _bp_component_growth)))

(event `/Game/WortelsGarden/Core/Sprites/BPI_SpriteActions.SetIsPickedUp`
  (params (`isPickedUp?` :type Boolean))
  (bind _bp_component_growth (`self.BP_Component_Growth`))
  (bind _growthtimer (`self.GrowthTimer`))
  (bind _output_get (set `self.isPickedUp?` `isPickedUp?`))
  (if _output_get
    (`/Game/WortelsGarden/Core/Sprites/BP_Component_Growth.PauseGrowth` _bp_component_growth)
    (`KismetSystemLibrary.PrintString` "pasue growth")
    (`SceneComponent.SetVisibility` _growthtimer false false)
    (else
      (`/Game/WortelsGarden/Core/Sprites/BP_Component_Growth.ResumeGrowth` _bp_component_growth)
      (`KismetSystemLibrary.PrintString` "resume growth")
      (if (`/Game/WortelsGarden/Core/Sprites/BP_Component_Growth.shouldGrow?` _bp_component_growth)
        (`SceneComponent.SetVisibility` _growthtimer true false)))))

(fn `GetHarvestableData`
  (returns (Harvestable :type Name) (MaxAmount :type Integer))
  (bind _bp_component_growth (`self.BP_Component_Growth`))
  (return (`/Game/WortelsGarden/Core/Sprites/BP_Component_Growth.Harvestable` _bp_component_growth) (`/Game/WortelsGarden/Core/Sprites/BP_Component_Growth.MaxHarvestableAmount` _bp_component_growth)))

(fn `SetSprites`
  (params (TopSprite :type "PaperSprite Object Reference") (BottomSprite :type "PaperSprite Object Reference"))
  (returns (`Success?` :type Boolean))
  (bind _returnvalue (`PaperSpriteComponent.SetSprite` (`self.Sprite`) BottomSprite))
  (bind _returnvalue_2 (`PaperSpriteComponent.SetSprite` (`self.SpriteFG`) TopSprite))
  (return (and _returnvalue_2 _returnvalue)))

(fn `SetUIScale`
  (bind _uiscale (message `/Game/WortelsGarden/Core/Player/BPI_GameMode.GetUIScale` (`GameplayStatics.GetGameMode`)))
  (bind _returnvalue (* _uiscale 75.0))
  (`WidgetComponent.SetDrawSize` (`self.Widget`) (`KismetMathLibrary.MakeVector2D` _returnvalue _returnvalue)))

(fn `Toggle Crop`
  (params (`isVisible?` :type Boolean))
  (`SceneComponent.SetHiddenInGame` (`self.SpriteFG`) (not `isVisible?`) false)
  (`SceneComponent.SetHiddenInGame` (`self.Sprite`) (not `isVisible?`) false)
  (`PrimitiveComponent.SetCollisionEnabled` (`self.Sprite`) (select `bool` (and `isVisible?` (`self.hasCollision?`)) :`false` "NoCollision" :`true` "QueryAndPhysics" :!type "ECollisionEnabled Enum")))

(fn `UserConstructionScript`
  (bind _rotatedspriteoffsett (`self.RotatedSpriteOffsett`))
  (`parent.UserConstructionScript`)
  (`SceneComponent.K2_SetRelativeLocation` (`self.SpriteBG`) (+ (* (`self.SpriteOffsett`) (`KismetMathLibrary.SelectVector` (-1.0 -1.0 -1.0) (1.0 1.0 1.0) (`self.isMirrored?`))) (select `int` (`self.Rotation`) :`0` (0.0 0.0 0.0) :`1` _rotatedspriteoffsett :`2` (0.0 0.0 0.0) :`3` _rotatedspriteoffsett)) false false)
  (set `self.DefaultRelativeLocation` (`SceneComponent.RelativeLocation` (`self.Sprite`)))
  (if (`self.isPickedUp?`)
    (`/Game/WortelsGarden/Core/Sprites/BP_Component_Growth.PauseGrowth` (`self.BP_Component_Growth`))
    (`KismetSystemLibrary.PrintString` "pausing growth because picked up")))