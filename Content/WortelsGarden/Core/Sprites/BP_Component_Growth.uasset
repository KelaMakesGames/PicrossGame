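; Growth component that advances its owning garden actor through sprite stages until it is ready to harvest.
; A looping timer splits growth time across the stages, sending top and bottom sprites and the harvest-ready state to the owner through messages.
; A second, pausable timer updates fractional progress from stage and timer elapsed time.
; Starting a harvest opens a puzzle widget sized by puzzle type; completing harvest is an empty stub.
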(event `self.ReceiveBeginPlay`
  (if (`self.shouldGrow?`)
    (`|ExecutionSequence`
      (:`then_0`
        ;[0.01891 0.01891 0.01891] Calculate Growth Stages
        (set `self.TotalGrowthStages` (- (`KismetArrayLibrary.Array_Length` (`self.BottomSprites`)) 1)))
      (:`then_1`
        ;[0.01891 0.01891 0.01891] Calculate Growth Time interval
        (set `self.GrowthIntervalTime` (/ (`self.GrowthTime`) (`self.TotalGrowthStages`))))
      (:`then_2`
        (bind _returnvalue (`KismetSystemLibrary.K2_SetTimer` null "Grow" (`self.GrowthIntervalTime`) true))
        (set `self.GrowthTimer` _returnvalue)
        (message `/Game/WortelsGarden/Core/Sprites/BPI_Growth.SetSprites` (`self.GetOwner`) (`|GetArrayItem` (`self.TopSprites`)) (`|GetArrayItem` (`self.BottomSprites`)))
        (bind _returnvalue_2 (`KismetSystemLibrary.K2_SetTimerDelegate` (delegate `GrowthUpdate`) 1.0 true))
        (bind _output_get (set `self.GrowthUpdateTimer` _returnvalue_2))
        (if (not (`self.isGrowthProgressShown?`))
          (`KismetSystemLibrary.K2_PauseTimerHandle` _output_get))))
    (elif (`self.isHarvestable?`)
      (set `self.isReadyToBeHarvested?` true)
      (message `/Game/WortelsGarden/Core/Sprites/BPI_Growth.SetReadyToBeHarvestable` (`self.GetOwner`)))))

(event `GrowthUpdate`
  (`self.SetGrowthProgress`))

(fn `CompleteHarvest`)

(fn `Grow`
  (bind _growthstage (`self.GrowthStage`))
  (`/Engine/EditorBlueprintResources/StandardMacros.IncrementInt` (`self.GrowthStage`)
    (:`  `
      (`|ExecutionSequence`
        (:`then_0`
          ;[0.01891 0.01891 0.01891] Set Sprites
          (message `/Game/WortelsGarden/Core/Sprites/BPI_Growth.SetSprites` (`self.GetOwner`) (`|GetArrayItem` (`self.TopSprites`) _growthstage) (`|GetArrayItem` (`self.BottomSprites`) _growthstage)))
        (:`then_1`
          (if (== (`self.GrowthStage`) (`self.TotalGrowthStages`))
            (set `self.isReadyToBeHarvested?` true)
            (message `/Game/WortelsGarden/Core/Sprites/BPI_Growth.SetReadyToBeHarvestable` (`self.GetOwner`))
            (`KismetSystemLibrary.K2_ClearAndInvalidateTimerHandle` (`self.GrowthTimer`))))))))

(fn `PauseGrowth`
  (if (`self.shouldGrow?`)
    (`KismetSystemLibrary.K2_PauseTimerHandle` (`self.GrowthTimer`))
    (`KismetSystemLibrary.K2_PauseTimerHandle` (`self.GrowthUpdateTimer`))))

(fn `PauseUpdateShowProgress`
  (`KismetSystemLibrary.K2_PauseTimerHandle` (`self.GrowthUpdateTimer`))
  (set `self.isGrowthProgressShown?` false))

(fn `ResumeGrowth`
  (if (`self.shouldGrow?`)
    (`KismetSystemLibrary.K2_UnPauseTimerHandle` (`self.GrowthTimer`))
    (`KismetSystemLibrary.K2_UnPauseTimerHandle` (`self.GrowthUpdateTimer`))))

(fn `ResumeUpdateShowProgress`
  (`KismetSystemLibrary.K2_UnPauseTimerHandle` (`self.GrowthUpdateTimer`))
  (set `self.isGrowthProgressShown?` true))

(fn `SetGrowthProgress`
  (returns (GrowthProgress :type "Float (double-precision)"))
  (bind _growthtimer (`self.GrowthTimer`))
  (bind _returnvalue (`KismetSystemLibrary.K2_GetTimerElapsedTimeHandle` _growthtimer))
  (bind _returnvalue_2 (`KismetMathLibrary.Conv_IntToDouble` (`self.TotalGrowthStages`)))
  (if (`self.isReadyToBeHarvested?`)
    (bind _output_get (set `self.GrowthProgress` 1.0))
    (return _output_get)
    (elif (`KismetSystemLibrary.K2_IsValidTimerHandle` _growthtimer)
      (bind _output_get_2 (set `self.GrowthProgress` (+ (* (/ _returnvalue (+ _returnvalue (`KismetSystemLibrary.K2_GetTimerRemainingTimeHandle` _growthtimer))) (/ 1.0 _returnvalue_2)) (/ (`KismetMathLibrary.Conv_IntToDouble` (`self.GrowthStage`)) _returnvalue_2))))
      (return _output_get_2)
      (else
        (bind _output_get_3 (set `self.GrowthProgress` 0.0))
        (return _output_get_3)))))

(fn `StartHarvest`
  (bind _returnvalue (`self.GetOwner`))
  (bind _returnvalue_2 (`GameplayStatics.GetPlayerController` 0))
  (switch `/Game/WortelsGarden/Core/Nonogram/ARCHIVE/E_PuzzleType` (`self.PuzzleType`)
    (:`NewEnumerator1`
      (bind _returnvalue_3 (`|CreateWidget` "/Game/WortelsGarden/Core/Nonogram/ARCHIVE/PuzzleBases/WBP_PuzzleBase.WBP_PuzzleBase_C" _returnvalue_2))
      (`UserWidget.AddToViewport` _returnvalue_3 100)
      (`/Game/WortelsGarden/Core/Nonogram/ARCHIVE/PuzzleBases/WBP_PuzzleBase.SETUP` _returnvalue_3 _returnvalue))
    (:`NewEnumerator3`
      (bind _returnvalue_4 (`|CreateWidget` "/Game/WortelsGarden/Core/Nonogram/ARCHIVE/PuzzleBases/WBP_PuzzleBase_15x15.WBP_PuzzleBase_15x15_C" _returnvalue_2))
      (`UserWidget.AddToViewport` _returnvalue_4 100)
      (`/Game/WortelsGarden/Core/Nonogram/ARCHIVE/PuzzleBases/WBP_PuzzleBase_15x15.SETUP` _returnvalue_4 _returnvalue))
    (:`NewEnumerator4`
      (bind _returnvalue_5 (`|CreateWidget` "/Game/WortelsGarden/Core/Nonogram/ARCHIVE/PuzzleBases/WBP_PuzzleBase_10x10.WBP_PuzzleBase_10x10_C" _returnvalue_2))
      (`UserWidget.AddToViewport` _returnvalue_5 100)
      (`/Game/WortelsGarden/Core/Nonogram/ARCHIVE/PuzzleBases/WBP_PuzzleBase_10x10.SETUP` _returnvalue_5 _returnvalue))))