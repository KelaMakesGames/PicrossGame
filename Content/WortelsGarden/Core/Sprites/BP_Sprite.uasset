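; Grid-based sprite actor for world objects that the player picks up, places, rotates or mirrors, cycles through variations, or stores in inventory.
; Cursor and click events on the Grid component check input mode and range, then message the player controller or pawn.
; Placement validity comes from per-cell line traces underground and an optional footprint box trace, tinting the grid while carried.
; The construction script applies collision, grid size, directional sprite, offset and inventory data.
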(event `/Game/WortelsGarden/Core/Sprites/BPI_Grid.FlashGrid`
  ;[0.01891 0.01891 0.01891] Grid
  (if (not (`self.isGridShown?`))
    (`self.ShowGrid` true)
    (`KismetSystemLibrary.Delay` 0.5)
    (`self.ShowGrid` false)))

(event `/Game/WortelsGarden/Core/Sprites/BPI_Grid.UpdatePlacability`
  ;[0.01891 0.01891 0.01891] Grid
  (`self.CheckIfPlacable`))

(event `/Game/WortelsGarden/Core/Sprites/BPI_Grid.SetSpriteCollision`
  ;[0.01891 0.01891 0.01891] Grid
  (`self.SetCollision`))

(event `/Game/WortelsGarden/Core/Sprites/BPI_Grid.UpdateGridColor`
  ;[0.01891 0.01891 0.01891] Grid
  (`self.SetGridColor`))

(event `/Game/WortelsGarden/Core/Sprites/BPI_Grid.SetSpriteGridCollision`
  (params (`hasGridCollision?` :type Boolean))
  ;[0.01891 0.01891 0.01891] Grid
  (set `self.hasGridCollision?` `hasGridCollision?`))

(event `/Game/WortelsGarden/Core/Sprites/BPI_Grid.SetCanShowGrid`
  (params (`canShowGrid?` :type Boolean))
  ;[0.01891 0.01891 0.01891] Grid
  (set `self.canShowGrid?` `canShowGrid?`))

(event `/Game/WortelsGarden/Core/Sprites/BPI_Grid.SetSpriteHasCollision`
  (params (`hasCollision?` :type Boolean))
  ;[0.01891 0.01891 0.01891] Grid
  (set `self.hasCollision?` `hasCollision?`))

(event `/Game/WortelsGarden/Core/Sprites/BPI_Grid.SetInGridInteractableRange`
  (params (`inRange?` :type Boolean))
  ;[0.01891 0.01891 0.01891] Grid
  (bind _output_get (set `self.inGridInteractableRange?` `inRange?`))
  (if _output_get
    (if (`self.isCursorOverGrid?`)
      (`self.ShowGrid` true)
      (else
        (`self.ShowGrid` false :!label _label)))
    (elif (not (`self.isPickedUp?`))
      (goto _label))))

(event `/Game/WortelsGarden/Core/Sprites/BPI_SpriteActions.SetIsPickedUp`
  (params (`isPickedUp?` :type Boolean))
  ;[0.01891 0.01891 0.01891] Grid
  (set `self.isPickedUp?` `isPickedUp?`))

(event `/Game/WortelsGarden/Core/Sprites/BPI_SpriteActions.UpdateMouseOverGrid`
  ;[0.01891 0.01891 0.01891] Cursor Over Grid
  (bind _inputmode (message `/Game/WortelsGarden/Core/Player/BPI_PlayerData.GetInputMode` (`GameplayStatics.GetPlayerController` 0) :!label _label_2))
  (bind _spriteunimpeded_ (`self.GetIfSpriteUnimpeded`))
  (if (and _spriteunimpeded_ (or (`|EnumEquality` _inputmode (`self.GridInteractInputMode`)) (`|EnumEquality` _inputmode "NewEnumerator3")))
    (set `self.isCursorOverGrid?` true)
    (if (and (`self.inGridInteractableRange?`) (`self.canShowGrid?`))
      (`self.ShowGrid` true)
      (message `/Game/WortelsGarden/Core/Player/BPI_PlayerData.SetGridShownActor` (`GameplayStatics.GetPlayerController` 0) self)
      (`self.CheckIfPlacable`))))

(event `self.Grid.OnBeginCursorOver`
  (params (TouchedComponent :type "PrimitiveComponent Object Reference"))
  ;[0.01891 0.01891 0.01891] Cursor Over Grid
  (goto _label_2))

(event `self.Grid.OnEndCursorOver`
  (params (TouchedComponent :type "PrimitiveComponent Object Reference"))
  (bind _returnvalue (`GameplayStatics.GetPlayerController` 0))
  ;[0.01891 0.01891 0.01891] Cursor Over Grid
  (set `self.isCursorOverGrid?` false)
  (if (not (`self.isPickedUp?`))
    (`self.ShowGrid` false)
    (bind _gridshownactor (message `/Game/WortelsGarden/Core/Player/BPI_PlayerData.GetGridShownActor` _returnvalue))
    (if (== _gridshownactor self)
      (message `/Game/WortelsGarden/Core/Player/BPI_PlayerData.SetGridShownActor` _returnvalue null))))

(event `self.Grid.OnClicked`
  (params (TouchedComponent :type "PrimitiveComponent Object Reference") (ButtonPressed :type "Key Structure"))
  (bind _returnvalue (`GameplayStatics.GetPlayerController` 0))
  (bind _returnvalue_2 (`self.K2_GetActorLocation`))
  (bind _keypressed (`self.KeyPressed`))
  ;[0.01891 0.01891 0.01891] Click Grid
  (set `self.KeyPressed` ButtonPressed)
  (bind _inputmode (message `/Game/WortelsGarden/Core/Player/BPI_PlayerData.GetInputMode` (`GameplayStatics.GetPlayerController` 0) :!label _label_3))
  (if (or (`|EnumEquality` _inputmode "NewEnumerator0") (`|EnumEquality` _inputmode "NewEnumerator3"))
    (bind _spriteunimpeded_ (`self.GetIfSpriteUnimpeded`))
    (if _spriteunimpeded_
      (if (`self.inGridInteractableRange?`)
        (if (== _keypressed "LeftMouseButton") :!label _label_4
          (if (`self.isPickedUp?`)
            (`self.CheckIfPlacable`)
            (if (`self.isValidPlacement?`)
              (set `self.isPickedUp?` false)
              (`self.SetCollision`)
              (`self.SetSpriteSortPriority` false)
              (message `/Game/WortelsGarden/Core/Sprites/BPI_Grid.Place` _returnvalue)
              (if (not (`self.inGridInteractableRange?`))
                (`self.ShowGrid` false))
              (else
                (`KismetSystemLibrary.PrintString` "not valid placement")))
            (elif (`self.canPickup?`)
              (set `self.isPickedUp?` true)
              (`self.SetCollision`)
              (`self.SetSpriteSortPriority` true)
              (bind _mouseoffset (`self.GetMouseOffset`))
              (message `/Game/WortelsGarden/Core/Sprites/BPI_Grid.Pickup` _returnvalue self _mouseoffset)))
          (elif (== _keypressed "RightMouseButton")
            (if (`self.isPickedUp?`)
              (bind _inputmode_2 (message `/Game/WortelsGarden/Core/Player/BPI_PlayerData.GetInputMode` (`GameplayStatics.GetPlayerController` 0)))
              (if (`|EnumEquality` _inputmode_2 "NewEnumerator3")
                (bind (_outhit _returnvalue_3) (`KismetSystemLibrary.LineTraceSingle` (+ _returnvalue_2 (-25.0 -25.0 100.0)) (+ _returnvalue_2 (-25.0 -25.0 -100.0)) "TraceTypeQuery3"))
                (if _returnvalue_3
                  (bind (_bblockinghit _binitialoverlap _time _distance _location _impactpoint _normal _impactnormal _physmat _hitactor) (`GameplayStatics.BreakHitResult` _outhit))
                  (`KismetSystemLibrary.PrintString` (`KismetStringLibrary.Concat_StrStr` "found: " (`KismetSystemLibrary.GetDisplayName` _hitactor)))
                  (bind _canbeaddedtoinventory_ (message `/Game/WortelsGarden/Core/Sprites/BPI_SpriteActions.GetCanBeAddedToInventory` _hitactor))
                  (if _canbeaddedtoinventory_
                    (message `/Game/WortelsGarden/Core/Sprites/BPI_Grid.Pickup` _hitactor null (0.0 0.0))
                    (else
                      (`self.Rotate` :!label _label_5)))
                  (else
                    (goto _label_5)))
                (else
                  (goto _label_5)))
              (elif (`self.canBeAddedToInventory?`)
                (if (`self.canPickup?`) :!label _label_6
                  (`self.AddToInventory`))
                (else
                  (goto _label_5))))))
        (elif (`self.isPickedUp?`)
          (goto _label_4))))
    (elif (and (`|EnumEquality` _inputmode "NewEnumerator4") (`self.canCustomizeVariation?`))
      (`self.IncrementVariation`))))

(event `/Game/WortelsGarden/Core/Sprites/BPI_Grid.Click`
  (params (ButtonPressed :type "Key Structure"))
  ;[0.01891 0.01891 0.01891] Click Grid
  (set `self.KeyPressed` ButtonPressed)
  (goto _label_3))

(event `/Game/WortelsGarden/Core/Sprites/BPI_Grid.Pickup`
  (params (PickedUpActor :type "Actor Object Reference") (MouseOffset :type "Vector2D Structure"))
  ;[0.01891 0.01891 0.01891] Click Grid
  (goto _label_6))

(event `/Game/WortelsGarden/Core/Sprites/BPI_Grid.Rotate`
  (bind _rotation (`self.Rotation`))
  ;[0.01891 0.01891 0.01891] Rotate
  (if (`self.canRotate?`)
    (if (== _rotation 3)
      (set `self.Rotation` 0)
      (else
        (`/Engine/EditorBlueprintResources/StandardMacros.IncrementInt` _rotation
          (:`  `
            _))))
    (`self.SetGrid`)
    (`self.SetSprite`)
    (`self.SetSpriteOffset`)
    (`self.UpdatePlacability`)
    (elif (`self.canMirror?`)
      (bind _isa (`/Engine/EditorBlueprintResources/StandardMacros.FlipFlop`)
        (:`A`
          _)
        (:`B`
          _))
      (`self.SetMirror` _isa))))

(event `SetSpriteSortPriority`
  (params (`PickedUp?` :type Boolean))
  (bind _sprite (`self.Sprite`))
  ;[0.01891 0.01891 0.01891] Sprite Sort Priority
  (if `PickedUp?`
    (set `self.DefaultSpriteSortPriority` (`PrimitiveComponent.TranslucencySortPriority` _sprite))
    (`PrimitiveComponent.SetTranslucentSortPriority` _sprite 5)
    (else
      (`PrimitiveComponent.SetTranslucentSortPriority` _sprite (`self.DefaultSpriteSortPriority`)))))

(event `/Game/WortelsGarden/Core/Sprites/BPI_SpriteActions.SetVariation`
  (params (Variation :type Integer))
  (set `self.Variation` Variation)
  (`self.SetSprite`))

(fn `AddToInventory`
  (bind _returnvalue (`GameplayStatics.GetPlayerController` 0))
  (bind (_inventoryitem_name _inventoryitem_displayname _inventoryitem_class _inventoryitem_variation _inventoryitem_amount _inventoryitem_stackable_ _inventoryitem_inputmode _inventoryitem_inventoryicon _inventoryitem_holditem) (break `/Game/WortelsGarden/Core/InventorySystem/S_InventoryItem` (`self.InventoryItem`)))
  (bind (_success_ _index) (message `/Game/WortelsGarden/Core/InventorySystem/BPI_InventorySystem.AddToContainer` (`GameplayStatics.GetPlayerPawn` 0) (make `/Game/WortelsGarden/Core/InventorySystem/S_InventoryItem` _inventoryitem_name _inventoryitem_displayname (`GameplayStatics.GetObjectClass` self) (`self.Variation`) _inventoryitem_amount _inventoryitem_stackable_ _inventoryitem_inputmode _inventoryitem_inventoryicon _inventoryitem_holditem)))
  (if (and _success_ (not (`self.IsActorBeingDestroyed` self)))
    (message `/Game/WortelsGarden/Core/InventorySystem/BPI_InventorySystem.UpdateContainer` _returnvalue _index false)
    (message `/Game/WortelsGarden/Core/Player/BPI_PlayerData.UpdateCurrentHUDSlot` _returnvalue)
    (`self.K2_DestroyActor`)))

(fn `BoxTraceGrid`
  (params (TraceChannel :type "ETraceTypeQuery Enum" :default "TraceTypeQuery1"))
  (returns (`hasAnyHit?` :type Boolean))
  (bind (_returnvalue_x _returnvalue_y) (`KismetMathLibrary.BreakVector` (`self.K2_GetActorLocation`)))
  (bind (_relativescale3d_x _relativescale3d_y) (`KismetMathLibrary.BreakVector` (`SceneComponent.RelativeScale3D` (`self.Grid`))))
  (bind _returnvalue (- (`self.RoundToClosest50` _returnvalue_y) (* _relativescale3d_y 25.0)))
  (bind _returnvalue_2 (- (`self.RoundToClosest50` _returnvalue_x) (- 50.0 (* _relativescale3d_x 25.0))))
  (bind (_outhit _returnvalue_3) (`KismetSystemLibrary.BoxTraceSingle` :`Start` (`KismetMathLibrary.MakeVector` _returnvalue_2 _returnvalue 100.0) :`End` (`KismetMathLibrary.MakeVector` _returnvalue_2 _returnvalue -100.0) :`HalfSize` (`KismetMathLibrary.MakeVector` (- (* _relativescale3d_x 25.0) 1.0) (- (* _relativescale3d_y 25.0) 1.0) 1.0) :`TraceChannel` TraceChannel :`TraceColor` (struct :`R` 1.0 :`G` 1.0 :`B` 1.0 :`A` 1.0) :`DrawTime` 1.0))
  (return _returnvalue_3))

(fn `CheckIfPlacable`
  (if (`self.inGridInteractableRange?`)
    (bind _isunderground_ (`self.CheckIfUnderground`))
    (if _isunderground_
      (bind _hashit_ (`self.Line Trace Grid` "TraceTypeQuery5"))
      (if _hashit_
        (if (not (`self.traceGridPlacability?`)) :!label _label
          (set `self.isValidPlacement?` true)
          (`self.SetGridColor` :!label _label_2)
          (else
            (bind _hasanyhit_ (`self.BoxTraceGrid` "TraceTypeQuery3"))
            (bind _returnvalue (not _hasanyhit_))
            (if (!= _returnvalue (`self.isValidPlacement?`))
              (set `self.isValidPlacement?` _returnvalue)
              (goto _label_2))))
        (else
          (set `self.isValidPlacement?` false)
          (goto _label_2)))
      (else
        (goto _label)))
    (else
      (set `self.isValidPlacement?` false)
      (goto _label_2))))

(fn `CheckIfUnderground`
  (returns (`isUnderground?` :type Boolean))
  (bind (_returnvalue_x _returnvalue_y) (`KismetMathLibrary.BreakVector` (`self.K2_GetActorLocation`)))
  (bind _output_get (set `self.isUnderground?` (> _returnvalue_y 600.0)))
  (return _output_get))

(fn `GetActorRotatability`
  (returns (`canRotate?` :type Boolean) (`canMirror?` :type Boolean))
  (return (`self.canRotate?`) (`self.canMirror?`)))

(fn `GetCanBeAddedToInventory`
  (returns (`canBeAddedToInventory?` :type Boolean))
  (return (`self.canBeAddedToInventory?`)))

(fn `GetIfSpriteUnimpeded`
  (returns (`SpriteUnimpeded?` :type Boolean))
  (bind (_pickedupactor _isvalidactor_) (message `/Game/WortelsGarden/Core/Sprites/BPI_Grid.GetPickedUpActor` (`GameplayStatics.GetPlayerController` 0)))
  (return (or (not _isvalidactor_) (== _pickedupactor self))))

(fn `GetisPickedUp?`
  (returns (`isPickedUp?` :type Boolean))
  (return (`self.isPickedUp?`)))

(fn `GetMouseOffset`
  (returns (MouseOffset :type "Vector2D Structure"))
  (bind (_returnvalue_x _returnvalue_y) (`KismetMathLibrary.BreakVector` (- (`self.K2_GetActorLocation`) (`PlayerController.DeprojectMousePositionToWorld` (`GameplayStatics.GetPlayerController` 0)))))
  (return (`KismetMathLibrary.MakeVector2D` _returnvalue_x _returnvalue_y)))

(fn `GetPickedUpActor`
  (returns (PickedUpActor :type "Actor Object Reference") (`isValidActor?` :type Boolean))
  (return null false))

(fn `IncrementVariation`
  (bind _result (`/Engine/EditorBlueprintResources/StandardMacros.IncrementInt` (`self.Variation`))
    (:`  `
      (if (>= _result (`KismetArrayLibrary.Array_Length` (`self.VariationSprites`)))
        (set `self.Variation` 0))
      (`self.SetVariation` (`self.Variation`)))))

(fn `Line Trace Grid`
  (params (TraceChannel :type "ETraceTypeQuery Enum" :default "TraceTypeQuery1") (`LookingForHit?` :type Boolean))
  (returns (`hasHit?` :type Boolean))
  (locals (`LOChasHit?` :type Boolean :default false))
  (bind (_returnvalue_x _returnvalue_y) (`KismetMathLibrary.BreakVector` (`self.K2_GetActorLocation`)))
  (bind (_relativescale3d_x _relativescale3d_y) (`KismetMathLibrary.BreakVector` (`SceneComponent.RelativeScale3D` (`self.Grid`))))
  (set `local.LOChasHit?` false)
  (for _index (range 1 (+ (`KismetMathLibrary.FTrunc` _relativescale3d_x) 1))
    (for _index_2 (range 1 (+ (`KismetMathLibrary.FTrunc` _relativescale3d_y) 1))
      (bind _returnvalue (+ (`self.RoundToClosest50` _returnvalue_x) (- (* _index 50.0) 75.0)))
      (bind _returnvalue_2 (+ (`self.RoundToClosest50` _returnvalue_y) (+ (* _index_2 -50.0) 25.0)))
      (bind (_outhit _returnvalue_3) (`KismetSystemLibrary.LineTraceSingle` (`KismetMathLibrary.MakeVector` _returnvalue _returnvalue_2 100.0) (`KismetMathLibrary.MakeVector` _returnvalue _returnvalue_2 -100.0) TraceChannel))
      (set `local.LOChasHit?` _returnvalue_3)
      (if (== `LookingForHit?` _returnvalue_3)
        (`KismetSystemLibrary.PrintString` (`KismetStringLibrary.Concat_StrStr` "BREAK " (`KismetMathLibrary.SelectString` (`KismetStringLibrary.Concat_StrStr` " HIT: " (`KismetSystemLibrary.GetDisplayName` (`.HitActor` (`GameplayStatics.BreakHitResult` _outhit)))) " no hit" _returnvalue_3)))
        (return `LookingForHit?`))))
  (return (`local.LOChasHit?`)))

(fn `SetCollision`
  (bind _grid (`self.Grid`))
  (`PrimitiveComponent.SetCollisionResponseToChannel` (`self.Sprite`) "ECC_Pawn" (select `bool` (`self.isPickedUp?`) :`false` (select `bool` (`self.hasCollision?`) :`false` "ECR_Overlap" :`true` "ECR_Block" :!type "ECollisionResponse Enum") :`true` "ECR_Ignore"))
  (`PrimitiveComponent.SetCollisionResponseToChannel` _grid "ECC_Visibility" (select `bool` (or (`self.canShowGrid?`) (`self.canGridTraceCursor?`)) :`false` "ECR_Ignore" :`true` "ECR_Block" :!type "ECollisionResponse Enum"))
  (`PrimitiveComponent.SetCollisionResponseToChannel` _grid "ECC_GameTraceChannel1" (select `bool` (`self.hasGridCollision?`) :`false` "ECR_Ignore" :`true` "ECR_Block" :!type "ECollisionResponse Enum")))

(fn `SetGrid`
  (bind _canrotategrid_ (`self.canRotateGrid?`))
  (bind (_gridsize_x _gridsize_y) (`KismetMathLibrary.BreakVector2D` (`self.GridSize`)))
  (bind _rotation (`self.Rotation`))
  (`SceneComponent.SetRelativeScale3D` (`self.Grid`) (`KismetMathLibrary.MakeVector` (`KismetMathLibrary.SelectFloat` (select `int` _rotation :`0` _gridsize_x :`1` _gridsize_y :`2` _gridsize_x :`3` _gridsize_y) _gridsize_x _canrotategrid_) (`KismetMathLibrary.SelectFloat` (select `int` _rotation :`0` _gridsize_y :`1` _gridsize_x :`2` _gridsize_y :`3` _gridsize_x) _gridsize_y _canrotategrid_) 1.0)))

(fn `SetGridColor`
  (`MeshComponent.SetVectorParameterValueOnMaterials` (`self.Grid`) "CLR" (`KismetMathLibrary.SelectVector` (`KismetMathLibrary.SelectVector` (`KismetMathLibrary.Conv_LinearColorToVector` (struct :`R` 0.12844 :`G` 1.0 :`A` 1.0)) (`KismetMathLibrary.Conv_LinearColorToVector` (struct :`R` 1.0 :`G` 0.054664 :`A` 1.0)) (`self.isValidPlacement?`)) (`KismetMathLibrary.Conv_LinearColorToVector` (struct :`R` 1.0 :`G` 1.0 :`B` 1.0 :`A` 1.0)) (`self.isPickedUp?`))))

(fn `SetMirror`
  (params (`Mirror?` :type Boolean))
  (`SceneComponent.SetRelativeScale3D` (`self.Sprite`) (`KismetMathLibrary.MakeVector` (`KismetMathLibrary.SelectFloat` -1.0 1.0 `Mirror?`) 1.0 1.0))
  (set `self.isMirrored?` `Mirror?`))

(fn `SetSprite`
  (bind _variation (`self.Variation`))
  (bind _variationsprites (`self.VariationSprites`))
  (bind (_output_top _output_right _output_bottom _output_left) (break `/Game/WortelsGarden/Core/Sprites/S_SpriteVariation` (`|GetArrayItem` _variationsprites _variation)))
  (if (`KismetArrayLibrary.Array_IsValidIndex` _variationsprites _variation)
    (`PaperSpriteComponent.SetSprite` (`self.Sprite`) (select `int` (`self.Rotation`) :`0` _output_top :`1` _output_right :`2` _output_bottom :`3` _output_left))))

(fn `SetSpriteOffset`
  (bind _rotatedspriteoffsett (`self.RotatedSpriteOffsett`))
  (`SceneComponent.K2_SetRelativeLocation` (`self.Sprite`) (+ (* (`self.SpriteOffsett`) (`KismetMathLibrary.SelectVector` (-1.0 -1.0 -1.0) (1.0 1.0 1.0) (`self.isMirrored?`))) (select `int` (`self.Rotation`) :`0` (0.0 0.0 0.0) :`1` _rotatedspriteoffsett :`2` (0.0 0.0 0.0) :`3` _rotatedspriteoffsett)) false false))

(fn `ShowGrid`
  (params (`isShown?` :type Boolean))
  (`SceneComponent.SetVisibility` (`self.Grid`) `isShown?` false)
  (`self.SetGridColor`))

(fn `ToggleMirror`
  (bind _isa (`/Engine/EditorBlueprintResources/StandardMacros.FlipFlop`)
    (:`A`
      _)
    (:`B`
      _))
  (`SceneComponent.SetRelativeScale3D` (`self.Sprite`) (`KismetMathLibrary.MakeVector` (`KismetMathLibrary.SelectFloat` -1.0 1.0 _isa) 1.0 1.0))
  (set `self.isMirrored?` _isa))

(fn `UserConstructionScript`
  (bind (_inventoryitem_name _inventoryitem_displayname _inventoryitem_class _inventoryitem_variation _inventoryitem_amount _inventoryitem_stackable_ _inventoryitem_inputmode _inventoryitem_inventoryicon _inventoryitem_holditem) (break `/Game/WortelsGarden/Core/InventorySystem/S_InventoryItem` (`self.InventoryItem`)))
  (bind (_gridsize_x _gridsize_y) (`KismetMathLibrary.BreakVector2D` (`self.GridSize`)))
  (`|ExecutionSequence`
    (:`then_0`
      (`self.CheckIfUnderground`)
      ;[0.01891 0.01891 0.01891] Collision
      (`self.SetCollision`))
    (:`then_1`
      ;[0.01891 0.01891 0.01891] GridPlacement
      (`self.ShowGrid` (`self.isGridShown?`))
      (`self.SetGrid`))
    (:`then_2`
      ;[0.01891 0.01891 0.01891] Variation
      (`self.SetSprite`))
    (:`then_3`
      ;[0.01891 0.01891 0.01891] Sprite Offsett
      (`self.SetSpriteOffset`))
    (:`then_4`
      ;[0.01891 0.01891 0.01891] Mirror
      (`SceneComponent.SetRelativeScale3D` (`self.Sprite`) (`KismetMathLibrary.MakeVector` (`KismetMathLibrary.SelectFloat` -1.0 1.0 (and (`self.isMirrored?`) (not (`self.MirrorAlongY?`)))) 1.0 (`KismetMathLibrary.SelectFloat` -1.0 1.0 (and (`self.isMirrored?`) (`self.MirrorAlongY?`)))))
      (if (and (`self.isMirrored?`) (`self.MirrorAlongY?`))
        (`SceneComponent.K2_AddLocalOffset` (`self.Sprite`) (`KismetMathLibrary.MakeVector` 0.0 0.0 (* _gridsize_y 50.0)) false false)))
    (:`then_5`
      (set `self.InventoryItem` (make `/Game/WortelsGarden/Core/InventorySystem/S_InventoryItem` _inventoryitem_name _inventoryitem_displayname (`GameplayStatics.GetObjectClass` self) (`self.Variation`) _inventoryitem_amount _inventoryitem_stackable_ _inventoryitem_inputmode _inventoryitem_inventoryicon (select `bool` (`self.useSpriteInInventoryItem?`) :`false` _inventoryitem_holditem :`true` (`PaperSpriteComponent.GetSprite` (`self.Sprite`))))))))