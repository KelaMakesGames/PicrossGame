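; BP_Sprite_Surface is a sprite actor that acts as a surface carrying an optional decoration, held in a child actor component.
; The construction script calls SetDeco, which stores the class and shows the component only when that class is valid.
; For a valid class it spawns the decoration, shifts it along local Y by its negated sprite offset, then messages it as on-surface with grid and sprite collision turned off.
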(event `self.ReceiveBeginPlay`
  (`parent.ReceiveBeginPlay`))

(fn `SetDeco`
  (params (Class :type "/Game/WortelsGarden/Core/Sprites/BP_Sprite_Deco Class Reference"))
  (bind _deco (`self.Deco`))
  (bind _childactor (`ChildActorComponent.ChildActor` _deco))
  (bind _output_get (set `self.DecoActorClass` Class))
  (bind _returnvalue (`KismetSystemLibrary.IsValidClass` _output_get))
  (`SceneComponent.SetVisibility` _deco _returnvalue false)
  (if _returnvalue
    (`ChildActorComponent.SetChildActorClass` _deco _output_get)
    (`self.SetDecoOffsett`)
    (message `/Game/WortelsGarden/Core/Sprites/BPI_Deco.SetOnSurface` _childactor true)
    (message `/Game/WortelsGarden/Core/Sprites/BPI_Grid.SetSpriteGridCollision` _childactor false)
    (message `/Game/WortelsGarden/Core/Sprites/BPI_Grid.SetSpriteHasCollision` _childactor false)
    (message `/Game/WortelsGarden/Core/Sprites/BPI_Grid.SetSpriteCollision` _childactor)))

(fn `SetDecoOffsett`
  (bind _offsett (message `/Game/WortelsGarden/Core/Sprites/BPI_Deco.GetSpriteOffsett` (`ChildActorComponent.ChildActor` (`self.Deco`))))
  (`SceneComponent.K2_AddLocalOffset` (`self.Deco`) (`KismetMathLibrary.MakeVector` 0.0 (`KismetMathLibrary.Conv_IntToDouble` (* _offsett -1))) false false))

(fn `UserConstructionScript`
  (`parent.UserConstructionScript`)
  (`|ExecutionSequence`
    (:`then_0`
      ;[0.01891 0.01891 0.01891] Decoration
      (`self.SetDeco` (`self.DecoActorClass`)))))