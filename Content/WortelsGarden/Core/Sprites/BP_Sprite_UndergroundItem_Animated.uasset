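; Animated underground item sprite Blueprint that shows one of several flipbook variations.
; The construction script picks the flipbook at the Variation index from FlipBookVariations, assigns it to the FlipBook component and hides the static Sprite.
; If that entry is invalid, it hides the FlipBook instead and prints a warning.
; The event graph has no active logic.
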(fn `UserConstructionScript`
  (bind _output (`|GetArrayItem` (`self.FlipBookVariations`) (`self.Variation`)))
  (`parent.UserConstructionScript`)
  (`/Engine/EditorBlueprintResources/StandardMacros.IsValid` _output
    (:`Is Valid`
      (`PaperFlipbookComponent.SetFlipbook` (`self.FlipBook`) _output)
      (`SceneComponent.SetVisibility` (`self.Sprite`) false false))
    (:`Is Not Valid`
      (`SceneComponent.SetVisibility` (`self.FlipBook`) false false)
      (`KismetSystemLibrary.PrintString` "UndergroudnItem_Animated > flipbook not valid"))))