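; Small plant sprite actor that sways in the wind and adds an extra rotation when RotateSprite fires.
; A slow WindRotate timeline drives sprite yaw, adding the value written by the Rotate timeline.
; A random stream seeded from actor X+Y jitters the sprite around its pivot and rotation offsets, refreshed on construction and placeability updates.
; Construction also forces the rotate overlap box's Z extent to 50 so rotation registers.
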(event `/Game/WortelsGarden/Core/Sprites/BPI_SpriteActions.RotateSprite`
  (bind _rotate (`self.Rotate`))
  (`TimelineComponent.SetPlayRate` _rotate 1.0)
  (if (`TimelineComponent.IsPlaying` _rotate)
    (bind (_direction _rotate_2) (`Timeline|Rotate` :!label _label)
      (:`Update`
        (set `self.AddativeRotation` _rotate_2)))
    (else
      (goto _label :!via `PlayFromStart`))))

(event `self.ReceiveBeginPlay`
  (bind _sprite (`self.Sprite`))
  (bind (_relativerotation_roll _relativerotation_pitch) (`KismetMathLibrary.BreakRotator` (`SceneComponent.RelativeRotation` _sprite)))
  (`TimelineComponent.SetPlayRate` (`self.WindRotate`) 0.1)
  (bind (_direction _rotate) (`Timeline|WindRotate`)
    (:`Update`
      (`SceneComponent.K2_SetRelativeRotation` _sprite (`KismetMathLibrary.MakeRotator` _relativerotation_roll _relativerotation_pitch (+ (* _rotate -1.0) (`self.AddativeRotation`))) false false))))

(event `/Game/WortelsGarden/Core/Sprites/BPI_Grid.UpdatePlacability`
  (`parent.UpdatePlacability`)
  (`self.SetSeedByLocation`)
  (`self.SetSpriteOffsetBySeed`))

(fn `SetSeedByLocation`
  (bind (_returnvalue_x _returnvalue_y) (`KismetMathLibrary.BreakVector` (`self.K2_GetActorLocation`)))
  (`KismetMathLibrary.SetRandomStreamSeed` (`self.RandomStream`) (`KismetMathLibrary.FTrunc` (+ _returnvalue_x _returnvalue_y))))

(fn `SetSpriteOffsetBySeed`
  (bind (_spritepivotoffsett_x _spritepivotoffsett_y) (`KismetMathLibrary.BreakVector2D` (`self.SpritePivotOffsett`)))
  (bind (_spritesize_x _spritesize_y) (`KismetMathLibrary.BreakVector2D` (`self.SpriteSize`)))
  (bind _rotatedspriteoffsett (`self.RotatedSpriteOffsett`))
  (bind (_offsettrange_x _offsettrange_y) (`KismetMathLibrary.BreakVector2D` (`self.OffsettRange`)))
  (bind (_returnvalue_x _returnvalue_y) (`KismetMathLibrary.BreakVector` (`KismetMathLibrary.RandomPointInBoundingBoxFromStream` (`self.RandomStream`) (0.0 0.0 0.0) (`KismetMathLibrary.MakeVector` _offsettrange_x _offsettrange_y))))
  (`SceneComponent.K2_SetRelativeLocation` (`self.Sprite`) (+ (+ (`self.SpriteOffsett`) (select `int` (`self.Rotation`) :`0` (0.0 0.0 0.0) :`1` _rotatedspriteoffsett :`2` (0.0 0.0 0.0) :`3` _rotatedspriteoffsett)) (`KismetMathLibrary.MakeVector` (+ (/ _spritepivotoffsett_x 5.12) _returnvalue_x) (+ (* (/ (- (/ _spritesize_y 2.0) _spritepivotoffsett_y) 5.12) -1.0) _returnvalue_y))) false false))

(fn `UserConstructionScript`
  (bind _rotateoverlapbox (`self.RotateOverlapBox`))
  (bind (_boxextent_x _boxextent_y) (`KismetMathLibrary.BreakVector` (`BoxComponent.BoxExtent` _rotateoverlapbox)))
  (`parent.UserConstructionScript`)
  (`self.SetSeedByLocation`)
  (`self.SetSpriteOffsetBySeed`)
  (`BoxComponent.SetBoxExtent` _rotateoverlapbox (`KismetMathLibrary.MakeVector` _boxextent_x _boxextent_y 50.0) true) ; for the rotate to register the box \nneeds the minimum z value of 50
)