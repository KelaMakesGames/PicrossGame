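; Decoration sprite actor that adapts translucency sorting and collision to whether it sits on a surface or on the ground.
; The construction script applies a sort distance offset and disables collision on surfaces; on the ground it clears the offset and makes collision optional.
; Sort priority comes from a surface value, a ground override or the default.
; SetonSurface reapplies sorting at runtime and toggles CanShowGrid, but leaves collision untouched.
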(event `/Game/WortelsGarden/Core/Sprites/BPI_Deco.SetOnSurface`
  (params (`onSurface?` :type Boolean))
  (`self.SetOnSurfaceLocal` `onSurface?`)
  (`self.SetSortPriority`)
  (set `self.canShowGrid?` (not `onSurface?`)))

(fn `GetSpriteOffsett`
  (returns (Offsett :type Integer))
  (return (`self.LocationOffset`)))

(fn `SetOnSurfaceLocal`
  (params (`onSurfacte?` :type Boolean))
  (bind _sprite (`self.Sprite`))
  (bind _output_get (set `self.onSurface?` `onSurfacte?`))
  (if _output_get
    (`PrimitiveComponent.SetTranslucencySortDistanceOffset` _sprite (`self.SortDistanceOffset`))
    (`KismetSystemLibrary.PrintString` "child actor!")
    (else
      (`PrimitiveComponent.SetTranslucencySortDistanceOffset` _sprite 0.0)
      (`KismetSystemLibrary.PrintString` "NO"))))

(fn `SetSortPriority`
  (`PrimitiveComponent.SetTranslucentSortPriority` (`self.Sprite`) (`KismetMathLibrary.SelectInt` (`self.OnSurfaceSortPriority`) (`KismetMathLibrary.SelectInt` (`self.OverrideSortPriorityOnGround`) (`self.DefaultSortPriority`) (and (`self.OverrideSortPriorityOnGround?`) (not (`self.onSurface?`)))) (`self.onSurface?`))))

(fn `UserConstructionScript`
  (bind _sprite (`self.Sprite`))
  (bind _sortdistanceoffset (`self.SortDistanceOffset`))
  (`parent.UserConstructionScript`)
  (`|ExecutionSequence`
    (:`then_0`
      ;[0.01891 0.01891 0.01891] Sort Distance
      (if (`self.onSurface?`)
        (`PrimitiveComponent.SetTranslucencySortDistanceOffset` _sprite _sortdistanceoffset)
        (`KismetSystemLibrary.PrintString` "child actor!")
        (set `self.ComputedSortDistance` _sortdistanceoffset)
        (else
          (`PrimitiveComponent.SetTranslucencySortDistanceOffset` _sprite 0.0)
          (`KismetSystemLibrary.PrintString` "NO")
          (set `self.ComputedSortDistance` 0.0))))
    (:`then_1`
      ;[0.01794 0.01794 0.01794] Surface Collision
      (if (`self.onSurface?`)
        (set `self.hasCollision?` false)
        (elif (`self.hasCollisionOnGround?`)
          (set `self.hasCollision?` true)
          (else
            (set `self.hasCollision?` false))))
      (`self.SetCollision`))
    (:`then_2`
      (`self.SetSortPriority`))))