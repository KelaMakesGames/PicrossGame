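; BP_Sprite_Carpet is the carpet sprite actor in WortelsGarden, a child Blueprint that relies on its parent for construction and grid interactable-range handling.
; Its own logic is in the Grid click event, which asks the player controller for the currently picked-up actor.
; If that actor is valid and is not the carpet itself, the click is forwarded to it through ClickMessage, so the carpet passes clicks through to held items.
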(event `/Game/WortelsGarden/Core/Sprites/BPI_Grid.SetInGridInteractableRange`
  (params (`inRange?` :type Boolean))
  (`parent.SetInGridInteractableRange` `inRange?`))

(event `self.Grid.OnClicked`
  (params (TouchedComponent :type "PrimitiveComponent Object Reference") (ButtonPressed :type "Key Structure"))
  (bind _pickedupactor (message `/Game/WortelsGarden/Core/Sprites/BPI_Grid.GetPickedUpActor` (`GameplayStatics.GetPlayerController` 0)))
  (`/Engine/EditorBlueprintResources/StandardMacros.IsValid` _pickedupactor
    (:`Is Valid`
      (if (!= _pickedupactor self)
        (message `/Game/WortelsGarden/Core/Sprites/BPI_Grid.Click` _pickedupactor ButtonPressed)))))

(fn `UserConstructionScript`
  (`parent.UserConstructionScript`))