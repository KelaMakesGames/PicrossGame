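; Sprite actor for an underground item in the garden that can be dug out.
; Construction rotates the sprite's yaw in 90-degree steps from a Rotation variable and sets the grid and sprite to block a custom trace channel.
; DigOut destroys the actor; the item drop gated by CanDropItem is still a debug-print placeholder.
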(fn `DigOut`
  (`KismetSystemLibrary.PrintString` "dig")
  (if (`self.canDropItem?`)
    (`KismetSystemLibrary.PrintString` "TO-DO: drop item"))
  (`self.K2_DestroyActor`))

(fn `UserConstructionScript`
  (bind _sprite (`self.Sprite`))
  (bind (_relativerotation_roll _relativerotation_pitch) (`KismetMathLibrary.BreakRotator` (`SceneComponent.RelativeRotation` _sprite)))
  (`parent.UserConstructionScript`)
  (`SceneComponent.K2_SetRelativeRotation` _sprite (`KismetMathLibrary.MakeRotator` _relativerotation_roll _relativerotation_pitch (`KismetMathLibrary.Conv_IntToDouble` (* (`self.Rotation`) 90))) false false)
  (`PrimitiveComponent.SetCollisionResponseToChannel` (`self.Grid`) "ECC_GameTraceChannel4" "ECR_Block")
  (`PrimitiveComponent.SetCollisionResponseToChannel` (`self.Sprite`) "ECC_GameTraceChannel4" "ECR_Block"))