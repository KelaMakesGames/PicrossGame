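; Auto-tiling sprite tile that picks its look and collision from neighbouring tiles of the same class.
; Line traces find orthogonal neighbours, whose presence pattern selects one of sixteen variations driving the sprite, foreground sprite, four edge box collisions and underground edge sprites.
; Corner sprites depend on left and right neighbours' variations, with diagonal tiles refreshed too.
; Tiles update at construction and BeginPlay; RemoveSelf hides the tile from traces and refreshes surrounding tiles before destruction.
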(event `self.ReceiveBeginPlay`
  (`parent.ReceiveBeginPlay`)
  (`self.UpdateTileVariation` false)
  (`self.SetAllBoxCollisions`))

(event `/Game/WortelsGarden/Core/Sprites/BPI_AutoTile.UpdateSurroundingTiles`
  (params (`FindSurroundingFencesFirst?` :type Boolean))
  (if `FindSurroundingFencesFirst?`
    (`self.FindSurroundingTiles` false))
  (for _array_element (`self.SurroundingTiles`)
    (message `/Game/WortelsGarden/Core/Sprites/BPI_AutoTile.UpdateTile` _array_element)))

(event `/Game/WortelsGarden/Core/Sprites/BPI_AutoTile.UpdateTile`
  (`self.UpdateTileVariation` false))

(fn `FindDiagonalTiles`
  (params (`showDebug?` :type Boolean))
  (bind (_returnvalue_x _returnvalue_y) (`KismetMathLibrary.BreakVector` (`self.K2_GetActorLocation`)))
  (`KismetArrayLibrary.Array_Clear` (`self.DiagonalSurroundingTiles`))
  (for _index (range 4)
    (bind _returnvalue (- (+ _returnvalue_x (select `int` _index :`0` -100.0 :`1` 100.0 :`2` 100.0 :`3` -100.0)) 0.0))
    (bind _returnvalue_2 (- (+ _returnvalue_y (select `int` _index :`0` -100.0 :`1` -100.0 :`2` 100.0 :`3` 100.0)) 50.0))
    (bind (_outhit _returnvalue_3) (`KismetSystemLibrary.LineTraceSingle` :`Start` (`KismetMathLibrary.MakeVector` _returnvalue _returnvalue_2 100.0) :`End` (`KismetMathLibrary.MakeVector` _returnvalue _returnvalue_2 -100.0) :`TraceChannel` "TraceTypeQuery5" :`DrawDebugType` "ForDuration" :`TraceColor` (struct :`R` 1.0 :`G` 1.0 :`B` 1.0 :`A` 1.0) :`DrawTime` 2.0))
    (if _returnvalue_3
      (bind (_bblockinghit _binitialoverlap _time _distance _location _impactpoint _normal _impactnormal _physmat _hitactor) (`GameplayStatics.BreakHitResult` _outhit))
      (if (== (`GameplayStatics.GetObjectClass` _hitactor) (`GameplayStatics.GetObjectClass` self))
        (`KismetArrayLibrary.Array_Set` (`self.DiagonalSurroundingTiles`) _index _hitactor true)
        (if `showDebug?`
          (message `/Game/WortelsGarden/Core/Sprites/BPI_Grid.FlashGrid` _hitactor))))))

(fn `FindSurroundingTiles`
  (params (`showDebug?` :type Boolean))
  (bind (_returnvalue_x _returnvalue_y) (`KismetMathLibrary.BreakVector` (`self.K2_GetActorLocation`)))
  (bind (_returnvalue_x_2 _returnvalue_y_2) (`KismetMathLibrary.BreakVector` (`self.K2_GetActorLocation`)))
  (`KismetArrayLibrary.Array_Clear` (`self.SurroundingTiles`))
  (set `self.hasTopNeighbour?` false)
  (set `self.hasRightNeighbour?` false)
  (set `self.hasBottomNeighbour?` false)
  (set `self.hasLeftNeighbour?` false)
  (for _index (range 4)
    (bind _returnvalue (- (+ _returnvalue_x_2 (select `int` _index :`0` 0.0 :`1` 100.0 :`2` 0.0 :`3` -100.0)) 0.0))
    (bind _returnvalue_2 (- (+ _returnvalue_y_2 (select `int` _index :`0` -100.0 :`1` 0.0 :`2` 100.0 :`3` 0.0)) 50.0))
    (bind (_outhit _returnvalue_3) (`KismetSystemLibrary.LineTraceSingle` :`Start` (`KismetMathLibrary.MakeVector` _returnvalue _returnvalue_2 100.0) :`End` (`KismetMathLibrary.MakeVector` _returnvalue _returnvalue_2 -100.0) :`TraceChannel` "TraceTypeQuery5" :`DrawDebugType` "ForDuration" :`TraceColor` (struct :`R` 1.0 :`G` 1.0 :`B` 1.0 :`A` 1.0) :`DrawTime` 2.0))
    (if _returnvalue_3
      (bind (_bblockinghit _binitialoverlap _time _distance _location _impactpoint _normal _impactnormal _physmat _hitactor) (`GameplayStatics.BreakHitResult` _outhit))
      (if (== (`GameplayStatics.GetObjectClass` _hitactor) (`GameplayStatics.GetObjectClass` self))
        (`KismetArrayLibrary.Array_Set` (`self.SurroundingTiles`) _index _hitactor true)
        (if `showDebug?`
          (message `/Game/WortelsGarden/Core/Sprites/BPI_Grid.FlashGrid` _hitactor))
        (switch `int` _index
          (:`0`
            (set `self.hasTopNeighbour?` true))
          (:`1`
            (set `self.hasRightNeighbour?` true))
          (:`2`
            (set `self.hasBottomNeighbour?` true))
          (:`3`
            (set `self.hasLeftNeighbour?` true))))))
  (if (and (`self.isUnderground?`) (<= _returnvalue_y 700.0))
    (set `self.hasTopNeighbour?` true)))

(fn `GetTileVariation`
  (returns (Variation :type Integer))
  (return (`self.Variation`)))

(fn `RemoveSelf`
  (`PrimitiveComponent.SetCollisionResponseToChannel` (`self.Sprite`) "ECC_GameTraceChannel3" "ECR_Ignore")
  (`PrimitiveComponent.SetCollisionResponseToChannel` (`self.Grid`) "ECC_GameTraceChannel3" "ECR_Ignore") ; prevent self from being seen by surrounding tiles
  (`self.UpdateSurroundingTiles` true)
  (`self.SetCorners` true)
  (`self.SetDiagonalCorners` false)
  (`self.K2_DestroyActor`))

(fn `SetAllBoxCollisions`
  (bind _variation (`self.Variation`))
  (bind _sprite (`self.Sprite`))
  (`|ExecutionSequence`
    (:`then_0`
      (bind _output_get (set `self.LeftCollision?` (select `int` _variation :`0` true :`1` true :`2` false :`3` false :`4` true :`5` true :`6` false :`7` false :`8` true :`9` true :`10` false :`11` false :`12` true :`13` true :`14` false :`15` false :`16` false)))
      (`self.SetBoxCollision` _output_get (`self.Box_Left`) (`self.Underground_Left`)))
    (:`then_1`
      (bind _output_get_2 (set `self.RightCollision?` (select `int` _variation :`0` true :`1` false :`2` false :`3` true :`4` true :`5` false :`6` false :`7` true :`8` true :`9` false :`10` false :`11` true :`12` true :`13` false :`14` false :`15` true :`16` false)))
      (`self.SetBoxCollision` _output_get_2 (`self.Box_Right`) (`self.Underground_Right`)))
    (:`then_2`
      (bind _output_get_3 (set `self.BottomCollision?` (select `int` _variation :`0` false :`1` false :`2` false :`3` false :`4` false :`5` false :`6` false :`7` false :`8` true :`9` true :`10` true :`11` true :`12` true :`13` true :`14` true :`15` true :`16` false)))
      (`self.SetBoxCollision` _output_get_3 (`self.Box_Rottom`) (`self.Underground_Bottom`)))
    (:`then_3`
      (bind _output_get_4 (set `self.TopCollision?` (select `int` _variation :`0` true :`1` true :`2` true :`3` true :`4` false :`5` false :`6` false :`7` false :`8` false :`9` false :`10` false :`11` false :`12` true :`13` true :`14` true :`15` true :`16` false)))
      (`self.SetBoxCollision` _output_get_4 (`self.Box_Top`)))
    (:`then_4`
      (`PrimitiveComponent.SetCollisionResponseToChannel` _sprite "ECC_GameTraceChannel3" "ECR_Block")
      (`PrimitiveComponent.SetCollisionResponseToChannel` _sprite "ECC_GameTraceChannel5" "ECR_Ignore")
      (`PrimitiveComponent.SetCollisionResponseToChannel` (`self.Grid`) "ECC_GameTraceChannel5" "ECR_Ignore")
      (`PrimitiveComponent.SetCollisionEnabled` _sprite "QueryOnly"))))

(fn `SetBoxCollision`
  (params (`CollisionEnabled?` :type Boolean) (Box :type "BoxComponent Object Reference") (UndergroundSprite :type "PaperSpriteComponent Object Reference"))
  (bind _isselector_ (`self.isSelector?`))
  (`PrimitiveComponent.SetCollisionEnabled` Box (select `bool` _isselector_ :`false` (select `bool` `CollisionEnabled?` :`false` "NoCollision" :`true` "QueryAndPhysics" :!type "ECollisionEnabled Enum") :`true` "NoCollision"))
  (`PrimitiveComponent.SetCollisionResponseToChannel` Box "ECC_Pawn" (select `bool` _isselector_ :`false` (select `bool` `CollisionEnabled?` :`false` "ECR_Ignore" :`true` "ECR_Block" :!type "ECollisionResponse Enum") :`true` "ECR_Ignore"))
  (`/Engine/EditorBlueprintResources/StandardMacros.IsValid` UndergroundSprite
    (:`Is Valid`
      (`SceneComponent.SetVisibility` UndergroundSprite (and `CollisionEnabled?` (not _isselector_)) false))))

(fn `SetCorners`
  (params (`skipFindingNeighbours?` :type Boolean))
  (locals (`wereCornersUpdated?` :type Boolean))
  (bind _output_top (break `/Game/WortelsGarden/Core/Sprites/S_SpriteVariation` (`|GetArrayItem` (`self.VariationSprites`) (`self.Variation`))))
  (set `local.wereCornersUpdated?` false)
  (if (not `skipFindingNeighbours?`)
    (`self.FindSurroundingTiles` false))
  (`|ExecutionSequence`
    (:`then_0`
      ;[0.01891 0.01891 0.01891] Left
      (if (`self.hasLeftNeighbour?`)
        (bind _variation (message `/Game/WortelsGarden/Core/Sprites/BPI_AutoTile.GetTileVariation` (`|GetArrayItem` (`self.SurroundingTiles`) 3)))
        (bind _returnvalue (and (select `int` _variation :`0` false :`1` true :`2` true :`3` false :`4` false :`5` false :`6` false :`7` false :`8` false :`9` false :`10` false :`11` false :`12` false :`13` true :`14` true :`15` false :`16` false) (select `int` (`self.Variation`) :`0` false :`1` false :`2` false :`3` false :`4` false :`5` false :`6` true :`7` true :`8` false :`9` false :`10` true :`11` true :`12` false :`13` false :`14` false :`15` false :`16` false)))
        (if (!= (`self.hasLeftCorner?`) _returnvalue)
          (set `local.wereCornersUpdated?` true))
        (set `self.hasLeftCorner?` _returnvalue)))
    (:`then_1`
      ;[0.01891 0.01891 0.01891] Right
      (if (`self.hasRightNeighbour?`)
        (bind _variation_2 (message `/Game/WortelsGarden/Core/Sprites/BPI_AutoTile.GetTileVariation` (`|GetArrayItem` (`self.SurroundingTiles`) 1)))
        (bind _returnvalue_2 (and (select `int` _variation_2 :`0` false :`1` false :`2` true :`3` true :`4` false :`5` false :`6` false :`7` false :`8` false :`9` false :`10` false :`11` false :`12` false :`13` false :`14` true :`15` true :`16` false) (select `int` (`self.Variation`) :`0` false :`1` false :`2` false :`3` false :`4` false :`5` true :`6` true :`7` false :`8` false :`9` true :`10` true :`11` false :`12` false :`13` false :`14` false :`15` false :`16` false)))
        (if (!= (`self.hasRightCorner?`) _returnvalue_2)
          (set `local.wereCornersUpdated?` true))
        (set `self.hasRightCorner?` _returnvalue_2)))
    (:`then_2`
      ;[0.01891 0.01891 0.01891] Set Sprite
      (`PaperSpriteComponent.SetSprite` (`self.Sprite`) (select `bool` (and (`self.hasLeftCorner?`) (`self.hasRightCorner?`)) :`false` (select `bool` (`self.hasRightCorner?`) :`false` (select `bool` (`self.hasLeftCorner?`) :`false` _output_top :`true` "/Game/WortelsGarden/Art/Environment/Underground/T_Tileset_Underground_Corner_Sprite_2.T_Tileset_Underground_Corner_Sprite_2") :`true` "/Game/WortelsGarden/Art/Environment/Underground/T_Tileset_Underground_Corner_Sprite_0.T_Tileset_Underground_Corner_Sprite_0") :`true` "/Game/WortelsGarden/Art/Environment/Underground/T_Tileset_Underground_Corner_Sprite_1.T_Tileset_Underground_Corner_Sprite_1")))))

(fn `SetDiagonalCorners`
  (params (`printDebug?` :type Boolean))
  (`self.FindDiagonalTiles` true)
  (for (_array_element _array_index) (`self.DiagonalSurroundingTiles`)
    (bind _asbp_sprite_tile (cast `/Game/WortelsGarden/Core/Sprites/BP_Sprite_Tile` _array_element))
    (`self.SetCorners` _asbp_sprite_tile false)
    (if `printDebug?`
      (bind _hasleftcorner_ (`/Game/WortelsGarden/Core/Sprites/BP_Sprite_Tile.hasLeftCorner?` _asbp_sprite_tile))
      (bind _hasrightcorner_ (`/Game/WortelsGarden/Core/Sprites/BP_Sprite_Tile.hasRightCorner?` _asbp_sprite_tile))
      (`KismetSystemLibrary.PrintString` (`KismetStringLibrary.Concat_StrStr` (select `int` _array_index :`0` "TOP LEFT: " :`1` "TOP RIGHT: " :`2` "BOTTOM RIGHT: " :`3` "BOTTOM LEFT: ") (`KismetSystemLibrary.GetDisplayName` _asbp_sprite_tile)) true true (`KismetMathLibrary.SelectColor` (struct :`G` 1.0 :`A` 1.0) (struct :`R` 1.0 :`A` 1.0) (or _hasleftcorner_ _hasrightcorner_)) 1.0)
      (`KismetSystemLibrary.PrintString` (`KismetStringLibrary.Concat_StrStr` "left: " (`KismetStringLibrary.Conv_BoolToString` _hasleftcorner_)) true true (`KismetMathLibrary.SelectColor` (struct :`G` 1.0 :`A` 1.0) (struct :`R` 1.0 :`A` 1.0) _hasleftcorner_) 1.0)
      (`KismetSystemLibrary.PrintString` (`KismetStringLibrary.Concat_StrStr` "right: " (`KismetStringLibrary.Conv_BoolToString` _hasrightcorner_)) true true (`KismetMathLibrary.SelectColor` (struct :`G` 1.0 :`A` 1.0) (struct :`R` 1.0 :`A` 1.0) _hasrightcorner_) 1.0))))

(fn `SetFGSprite`
  (bind _fgvariations (`self.FGVariations`))
  (bind _variation (`self.Variation`))
  ;[0.01891 0.01891 0.01891] Foreground Sprite
  (if (`KismetArrayLibrary.Array_IsValidIndex` _fgvariations _variation)
    (`PaperSpriteComponent.SetSprite` (`self.SpriteFG`) (`|GetArrayItem` _fgvariations _variation))))

(fn `SetTileType`
  (for _index (range 16)
    (if (`KismetArrayLibrary.Array_Identical` (`|MakeArray` (`self.hasTopNeighbour?`) (`self.hasRightNeighbour?`) (`self.hasBottomNeighbour?`) (`self.hasLeftNeighbour?`)) (select `int` _index :`0` (`|MakeArray` false false true false) :`1` (`|MakeArray` false true true false) :`2` (`|MakeArray` false true true true) :`3` (`|MakeArray` false false true true) :`4` (`|MakeArray` true false true false) :`5` (`|MakeArray` true true true false) :`6` (`|MakeArray` true true true true) :`7` (`|MakeArray` true false true true) :`8` (`|MakeArray` true false false false) :`9` (`|MakeArray` true true false false) :`10` (`|MakeArray` true true false true) :`11` (`|MakeArray` true false false true) :`12` (`|MakeArray` false false false false) :`13` (`|MakeArray` false true false false) :`14` (`|MakeArray` false true false true) :`15` (`|MakeArray` false false false true)))
      (if (!= (`self.Variation`) _index)
        (bind _output_get (set `self.Variation` _index))
        (bind _output_top (break `/Game/WortelsGarden/Core/Sprites/S_SpriteVariation` (`|GetArrayItem` (`self.VariationSprites`) _output_get)))
        (`PaperSpriteComponent.SetSprite` (`self.Sprite`) _output_top)
        (`self.SetCorners` false)
        (`self.SetFGSprite`)
        (`self.SetAllBoxCollisions`)
        (break)))))

(fn `UpdateTileVariation`
  (params (`showDebug?` :type Boolean))
  (`self.FindSurroundingTiles` `showDebug?`)
  (`self.SetTileType`))

(fn `UserConstructionScript`
  (`parent.UserConstructionScript`)
  (`self.UpdateTileVariation` false)
  (`self.SetCorners` true)
  (`self.SetDiagonalCorners` false)
  (`self.SetFGSprite`)
  (`self.SetAllBoxCollisions`)
  (`self.FindDiagonalTiles` false)
  (`SceneComponent.SetVisibility` (`self.Grid`) false false))