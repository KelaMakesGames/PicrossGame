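; BP_DigSelector is the underground dig/fill cursor: clicking it spends player energy to spawn a dug tile or remove an existing one.
; UpdateSelector shows it only underground near the player, traces for a tile to choose dig or fill, and sets a valid or invalid sprite.
; Placement requires a clear box trace and, for digging, an orthogonally adjacent tile.
; Digging also unearths any item under the mouse and refreshes neighbouring tiles.
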(event `self.BG.OnClicked`
  (params (TouchedComponent :type "PrimitiveComponent Object Reference") (ButtonPressed :type "Key Structure"))
  (bind _worldlocation (`PlayerController.DeprojectMousePositionToWorld` (`GameplayStatics.GetPlayerController` 0)))
  (bind _worldlocation_2 (`PlayerController.DeprojectMousePositionToWorld` (`GameplayStatics.GetPlayerController` 0)))
  (bind _energy (message `/Game/WortelsGarden/Core/Player/BPI_PlayerData.GetEnergy` (`GameplayStatics.GetPlayerController` 0)))
  (if (>= _energy 1.0)
    (`KismetSystemLibrary.PrintString` "dig")
    (bind _diglocation (message `/Game/WortelsGarden/Core/Player/BPI_PlayerData.GetDigLocation` (`GameplayStatics.GetPlayerController` 0)))
    (if (and (> (`.Y` (`KismetMathLibrary.BreakVector2D` _diglocation)) 700.0) (`self.canPlaceTile?`))
      (if (`self.Dig?`)
        (bind _outhit (`KismetSystemLibrary.LineTraceSingle` (`KismetMathLibrary.MakeVector` (.x _worldlocation_2) (.y _worldlocation_2) 100.0) (`KismetMathLibrary.MakeVector` (.x _worldlocation_2) (.y _worldlocation_2) -100.0) "TraceTypeQuery6"))
        (bind _asbp_sprite_underground_item (cast `/Game/WortelsGarden/Core/Sprites/BP_Sprite_UndergroundItem` (`.HitActor` (`GameplayStatics.BreakHitResult` _outhit)))
          (:`then`
            (`/Game/WortelsGarden/Core/Sprites/BP_Sprite_UndergroundItem.DigOut` _asbp_sprite_underground_item))
          (:`CastFailed`
            _))
        (bind _returnvalue (`|SpawnActorFromClass` "/Game/WortelsGarden/Core/Sprites/BP_Sprite_Tile.BP_Sprite_Tile_C" (`KismetMathLibrary.MakeTransform` (`KismetMathLibrary.MakeVector` (`KismetMathLibrary.BreakVector2D` _diglocation) (`.Y` (`KismetMathLibrary.BreakVector2D` _diglocation)) -1.0)) "Undefined" "MultiplyWithRoot" null null))
        (`/Game/WortelsGarden/Core/Sprites/BP_Sprite_Tile.UpdateSurroundingTiles` _returnvalue true)
        (`/Game/WortelsGarden/Core/Sprites/BP_Sprite_Tile.SetCorners` _returnvalue true)
        (`/Game/WortelsGarden/Core/Sprites/BP_Sprite_Tile.SetDiagonalCorners` _returnvalue false)
        (`self.UpdateSelector`)
        (else
          (bind _outhit_2 (`KismetSystemLibrary.LineTraceSingle` (`KismetMathLibrary.MakeVector` (.x _worldlocation) (.y _worldlocation) 100.0) (`KismetMathLibrary.MakeVector` (.x _worldlocation) (.y _worldlocation) -100.0) "TraceTypeQuery5"))
          (bind _asbp_sprite_tile (cast `/Game/WortelsGarden/Core/Sprites/BP_Sprite_Tile` (`.HitActor` (`GameplayStatics.BreakHitResult` _outhit_2))))
          (`/Game/WortelsGarden/Core/Sprites/BP_Sprite_Tile.RemoveSelf` _asbp_sprite_tile)
          (`self.UpdateSelector`)))
      (message `/Game/WortelsGarden/Core/Player/BPI_PlayerData.RemoveEnergy` (`GameplayStatics.GetPlayerController` 0) 0.5)
      (else
        (`KismetSystemLibrary.PrintString` "cannot dig/fill" :!label _label)))
    (else
      (goto _label))))

(fn `CheckDiggability`
  (returns (`canDig?` :type Boolean))
  (locals (`foundHit?` :type Boolean))
  (bind (_returnvalue_x _returnvalue_y) (`KismetMathLibrary.BreakVector` (`self.K2_GetActorLocation`)))
  (for _index (range 4)
    (bind _returnvalue (- (+ _returnvalue_x (select `int` _index :`0` 0.0 :`1` 100.0 :`2` 0.0 :`3` -100.0)) 0.0))
    (bind _returnvalue_2 (- (+ _returnvalue_y (select `int` _index :`0` -100.0 :`1` 0.0 :`2` 100.0 :`3` 0.0)) 50.0))
    (bind (_outhit _returnvalue_3) (`KismetSystemLibrary.LineTraceSingle` :`Start` (`KismetMathLibrary.MakeVector` _returnvalue _returnvalue_2 100.0) :`End` (`KismetMathLibrary.MakeVector` _returnvalue _returnvalue_2 -100.0) :`TraceChannel` "TraceTypeQuery5" :`DrawDebugType` "ForDuration" :`TraceColor` (struct :`R` 1.0 :`G` 1.0 :`B` 1.0 :`A` 1.0) :`DrawTime` 2.0))
    (if _returnvalue_3
      (set `local.foundHit?` true)
      (return true)))
  (return false))

(fn `UpdateSelector`
  (bind _returnvalue (`self.K2_GetActorLocation`))
  (bind (_returnvalue_x _returnvalue_y) (`KismetMathLibrary.BreakVector` (+ _returnvalue (0.0 -50.0 0.0))))
  (bind _returnvalue_2 (and (> (.y _returnvalue) 700.0) (< (`self.GetDistanceTo` (`GameplayStatics.GetPlayerPawn` 0)) 180.0)))
  (`SceneComponent.SetVisibility` (`self.BG`) _returnvalue_2 false)
  (if _returnvalue_2
    (bind (_outhit _returnvalue_3) (`KismetSystemLibrary.LineTraceSingle` (`KismetMathLibrary.MakeVector` _returnvalue_x _returnvalue_y 100.0) (`KismetMathLibrary.MakeVector` _returnvalue_x _returnvalue_y -100.0) "TraceTypeQuery5"))
    (bind _diglocation (message `/Game/WortelsGarden/Core/Player/BPI_PlayerData.GetDigLocation` (`GameplayStatics.GetPlayerController` 0)))
    (bind _returnvalue_4 (not _returnvalue_3))
    (bind _canplacetile_ (`self.UpdateTilePlacability` _diglocation _returnvalue_4))
    (bind _energy (message `/Game/WortelsGarden/Core/Player/BPI_PlayerData.GetEnergy` (`GameplayStatics.GetPlayerController` 0)))
    (bind _returnvalue_5 (and _canplacetile_ (>= _energy 0.5)))
    (set `self.canPlaceTile?` _returnvalue_5)
    (bind _output_get (set `self.Dig?` _returnvalue_4))
    (`PaperSpriteComponent.SetSprite` (`self.BG`) (select `bool` _returnvalue_5 :`false` (select `bool` _output_get :`false` "/Game/WortelsGarden/Art/Environment/Underground/T_DigFill_Invalid_Sprite.T_DigFill_Invalid_Sprite" :`true` "/Game/WortelsGarden/Art/Environment/Underground/T_Dig_Invalid_Sprite.T_Dig_Invalid_Sprite" :!type "PaperSprite Object Reference") :`true` (select `bool` _output_get :`false` "/Game/WortelsGarden/Art/Environment/Underground/T_DigFill_Sprite.T_DigFill_Sprite" :`true` "/Game/WortelsGarden/Art/Environment/Underground/T_Dig_Sprite.T_Dig_Sprite" :!type "PaperSprite Object Reference")))
    (else
      (set `self.canPlaceTile?` false)
      (set `self.Dig?` false))))

(fn `UpdateTilePlacability`
  (params (DigLocation :type "Vector2D Structure") (`checkDiggability?` :type Boolean))
  (returns (`canPlaceTile?` :type Boolean) (`canDig?` :type Boolean))
  (bind _returnvalue (- DigLocation_Y 50.0))
  (bind (_outhit _returnvalue_2) (`KismetSystemLibrary.BoxTraceSingle` (`KismetMathLibrary.MakeVector` DigLocation_X _returnvalue 100.0) (`KismetMathLibrary.MakeVector` DigLocation_X _returnvalue -100.0) (40.0 40.0 40.0) (struct) "TraceTypeQuery7"))
  (bind _returnvalue_3 (not _returnvalue_2))
  (if (and _returnvalue_3 `checkDiggability?`)
    (bind _candig_ (`self.CheckDiggability`))
    (return _candig_ _candig_)
    (else
      (if _returnvalue_2
        (bind (_bblockinghit _binitialoverlap _time _distance _location _impactpoint _normal _impactnormal _physmat _hitactor) (`GameplayStatics.BreakHitResult` _outhit))
        (bind _returnvalue_4 (`GameplayStatics.GetObjectClass` _hitactor))
        (if (and (!= _hitactor (`GameplayStatics.GetPlayerPawn` 0)) (or (== _returnvalue_4 "/Game/WortelsGarden/Placeables/BP_Sprite_UndergroundBorder_Right.BP_Sprite_UndergroundBorder_Right_C") (== _returnvalue_4 "/Game/WortelsGarden/Placeables/BP_Sprite_UndergroundBorder_Lower.BP_Sprite_UndergroundBorder_Lower_C")))
          (`SceneComponent.SetVisibility` (`self.BG`) false false)
          (`KismetSystemLibrary.PrintString` "set dig selector invisible (meant for environment borders)")))
      (return _returnvalue_3 false))))

(fn `UserConstructionScript`
  (set `self.DefaultLocation` (`self.K2_GetActorLocation`)))