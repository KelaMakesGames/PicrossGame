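; BP_GroundBlockingVolume is a box volume that blocks Pawns on ground that has no hole.
; The construction script sizes the box, then runs UpdateCollision.
; UpdateCollision line-traces vertically at a Y offset; hitting BP_Sprite_GroundHole disables and hides the box and sets HasGroundHole, while other hits make it a query-only Pawn blocker.
; With no hit, collision is disabled but the box stays unhidden.
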(fn `UpdateCollision`
  (bind (_returnvalue_x _returnvalue_y) (`KismetMathLibrary.BreakVector` (`self.K2_GetActorLocation`)))
  (bind _box (`self.Box`))
  (bind _box_2 (`self.Box`))
  (bind _returnvalue (- _returnvalue_y 50.0))
  (bind (_outhit _returnvalue_2) (`KismetSystemLibrary.LineTraceSingle` (`KismetMathLibrary.MakeVector` _returnvalue_x _returnvalue 100.0) (`KismetMathLibrary.MakeVector` _returnvalue_x _returnvalue -100.0) "TraceTypeQuery8"))
  (if _returnvalue_2
    (bind _returnvalue_3 (== (`GameplayStatics.GetObjectClass` (`.HitActor` (`GameplayStatics.BreakHitResult` _outhit))) "/Game/WortelsGarden/Core/Sprites/BP_Sprite_GroundHole.BP_Sprite_GroundHole_C"))
    (`PrimitiveComponent.SetCollisionEnabled` _box (select `bool` _returnvalue_3 :`false` "QueryOnly" :`true` "NoCollision" :!type "ECollisionEnabled Enum"))
    (`PrimitiveComponent.SetCollisionResponseToChannel` _box "ECC_Pawn" (select `bool` _returnvalue_3 :`false` "ECR_Block" :`true` "ECR_Ignore" :!type "ECollisionResponse Enum"))
    (`SceneComponent.SetHiddenInGame` _box_2 _returnvalue_3 false)
    (set `self.hasGroundHole?` _returnvalue_3)
    (else
      (`PrimitiveComponent.SetCollisionEnabled` _box "NoCollision")
      (`PrimitiveComponent.SetCollisionResponseToChannel` _box "ECC_Pawn" "ECR_Block")
      (`SceneComponent.SetHiddenInGame` _box_2 _returnvalue_2 false)
      (set `self.hasGroundHole?` _returnvalue_2))))

(fn `UserConstructionScript`
  (`BoxComponent.SetBoxExtent` (`self.Box`) (`self.BoxExtent`) true)
  (`self.UpdateCollision`))