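; Container component that stores an inventory as a capacity-limited array of item structs, with add and remove operations.
; Stackable items merge into a slot matching name and variation; others take the first zero-amount slot or extend the array.
; Removal by name or by index decrements the amount, clears emptied slots in place to keep indices stable, and reports any shortfall left to remove.
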(fn `AddToInventory`
  (params (InventoryItem :type "/Game/WortelsGarden/Core/InventorySystem/S_InventoryItem Structure"))
  (returns (`success?` :type Boolean) (Index :type Integer))
  (bind (_name _displayname _class _variation _amount _stackable_ _inputmode _inventoryicon _holditem) (break `/Game/WortelsGarden/Core/InventorySystem/S_InventoryItem` InventoryItem))
  (bind ((`Name_11_3B3AAA62F34C78C7B0F22EA2965F892E` _name_2) (`Variation_10_517AB4EE374B384BA9C0A79A530094FE` _variation_2)) (break `/Game/WortelsGarden/Core/InventorySystem/S_InventoryItem` InventoryItem))
  (bind _inventory (`self.Inventory`))
  (bind _inventory_2 (`self.Inventory`))
  (bind _isfull_ (`self.CheckIfInventoryFull`))
  (if _isfull_
    (return false 0)
    (else
      (if (`.Stackable?_17_ED62BDE1D8401D98904F1C9943E3912F` (break `/Game/WortelsGarden/Core/InventorySystem/S_InventoryItem` InventoryItem))
        (bind (_isfound_ _itemindex) (`self.FindInInventory` _name_2 _variation_2))
        (if _isfound_
          (bind (_output_name _output_displayname _output_class _output_variation _output_amount) (break `/Game/WortelsGarden/Core/InventorySystem/S_InventoryItem` (`|GetArrayItem` _inventory_2 _itemindex)))
          (`KismetArrayLibrary.Array_Set` _inventory_2 _itemindex (make `/Game/WortelsGarden/Core/InventorySystem/S_InventoryItem` _name _displayname _class _variation (+ _output_amount _amount) _stackable_ _inputmode _inventoryicon _holditem) true)
          (return true _itemindex)
          (else
            _)))
      (bind (_foundindex_ _index) (`self.FindEmptyIndex`))
      (if _foundindex_
        (`KismetArrayLibrary.Array_Set` _inventory _index InventoryItem true)
        (return true _index)
        (else
          (bind _returnvalue (`KismetArrayLibrary.Array_Add` _inventory InventoryItem))
          (return true _returnvalue))))))

(fn `AddToInventoryByIndex`
  (params (Item :type "/Game/WortelsGarden/Core/InventorySystem/S_InventoryItem Structure") (Index :type Integer))
  (returns (`success?` :type Boolean))
  (`KismetArrayLibrary.Array_Set` (`self.Inventory`) Index Item true)
  (return true))

(fn `CheckIfInventoryFull`
  (returns (`isFull?` :type Boolean))
  (locals (`HasEmptyIndex?` :type Boolean))
  (if (`self.CheckIfInventoryFullByLength`)
    (bind _foundindex_ (`self.FindEmptyIndex`))
    (return (not _foundindex_))
    (else
      (return false))))

(fn `FindEmptyIndex`
  (returns (`FoundIndex?` :type Boolean) (Index :type Integer))
  (locals (`FoundFirst?` :type Boolean) (FirstEmptyIndex :type Integer))
  (bind _inventory (`self.Inventory`))
  (bind _returnvalue (`KismetArrayLibrary.Array_Length` _inventory))
  (for (_array_element _array_index) _inventory
    (if (== (`.Amount_9_18C02BD3F7475CFB8251C3A4A542074E` (break `/Game/WortelsGarden/Core/InventorySystem/S_InventoryItem` _array_element)) 0)
      (set `local.FirstEmptyIndex` _array_index)
      (set `local.FoundFirst?` true)
      (break)))
  (if (`local.FoundFirst?`)
    (return (`local.FoundFirst?`) (`local.FirstEmptyIndex`))
    (elif (< _returnvalue (`self.InventoryCapacity`))
      (return true _returnvalue)
      (else
        (return false -1)))))

(fn `FindInInventory`
  (params (Name :type Name) (Variation :type Integer))
  (returns (`isFound?` :type Boolean) (ItemIndex :type Integer))
  (locals (`TEMPisFound?` :type Boolean) (TEMPItemIndex :type Integer :default -1))
  (for (_array_element _array_index) (`self.Inventory`)
    (if (and (== (break `/Game/WortelsGarden/Core/InventorySystem/S_InventoryItem` _array_element) Name) (== (`.Variation_10_517AB4EE374B384BA9C0A79A530094FE` (break `/Game/WortelsGarden/Core/InventorySystem/S_InventoryItem` _array_element)) Variation))
      (set `local.TEMPisFound?` true)
      (set `local.TEMPItemIndex` _array_index)
      (break)))
  (return (`local.TEMPisFound?`) (`local.TEMPItemIndex`)))

(fn `RemoveFromInventory`
  (params (Name :type Name) (Variation :type Integer) (Amount :type Integer))
  (returns (`success?` :type Boolean) (AmountLeftToRemove :type Integer))
  (bind _inventory (`self.Inventory`))
  (bind (_isfound_ _itemindex) (`self.FindInInventory` Name Variation))
  (if _isfound_
    (bind _output (`|GetArrayItem` (`self.Inventory`) _itemindex))
    (bind ((`Amount_9_18C02BD3F7475CFB8251C3A4A542074E` _amount)) (break `/Game/WortelsGarden/Core/InventorySystem/S_InventoryItem` _output))
    (bind _returnvalue (- _amount Amount))
    (`/Engine/EditorBlueprintResources/StandardMacros.CompareInt` _returnvalue
      (:`>`
        (bind (_name _displayname _class _variation _amount_2 _stackable_ _inputmode _inventoryicon _holditem) (break `/Game/WortelsGarden/Core/InventorySystem/S_InventoryItem` _output))
        (`KismetArrayLibrary.Array_Set` _inventory _itemindex (make `/Game/WortelsGarden/Core/InventorySystem/S_InventoryItem` _name _displayname _class _variation _returnvalue _stackable_ _inputmode _inventoryicon _holditem))
        (return true 0))
      (:`==`
        (`KismetArrayLibrary.Array_Set` _inventory _itemindex) ; clear array elem
        (return true 0))
      (:`<`
        (`KismetArrayLibrary.Array_Set` _inventory _itemindex)
        (return true (- Amount _amount))))
    (else
      (return false 0) ; item not in inventory, \ncannot remove
    )))

(fn `RemoveFromInventoryByIndex`
  (params (Index :type Integer) (Amount :type Integer))
  (returns (AmountLeftToRemove :type Integer))
  (locals (AmountLeft :type Integer))
  (bind _inventory (`self.Inventory`))
  (bind (_output_name _output_displayname _output_class _output_variation _output_amount _output_stackable_ _output_inputmode _output_inventoryicon _output_holditem) (break `/Game/WortelsGarden/Core/InventorySystem/S_InventoryItem` (`|GetArrayItem` (`self.Inventory`) Index)))
  (`/Engine/EditorBlueprintResources/StandardMacros.CompareInt` _output_amount Amount
    (:`>`
      (`KismetArrayLibrary.Array_Set` _inventory Index (make `/Game/WortelsGarden/Core/InventorySystem/S_InventoryItem` _output_name _output_displayname _output_class _output_variation (- _output_amount Amount) _output_stackable_ _output_inputmode _output_inventoryicon _output_holditem))
      (set `local.AmountLeft` 0 :!label _label))
    (:`==`
      (`KismetArrayLibrary.Array_Set` _inventory Index)
      (goto _label))
    (:`<`
      (set `local.AmountLeft` (- Amount _output_amount))
      (`KismetArrayLibrary.Array_Set` _inventory Index)))
  (return (`local.AmountLeft`)))